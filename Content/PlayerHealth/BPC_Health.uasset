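; Health component for the first-person character that handles damage, regeneration and death, updating the HUD and opening the death menu at zero health.
; Damage is divided by a defence level that climbs with hits taken at low health, while the first lethal heavy hit leaves 1 HP.
; Regeneration applies growing negative damage after a retriggerable delay, looping back through the damage handler.
; Tick polls for death, and key 3 deals test damage.
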(event `self.ReceiveTick`
  (params (DeltaSeconds :type "Float (single-precision)"))
  (if (and (not (`self.IsDead`)) (== (`self.Health`) 0.0))
    (set `self.IsDead` true)
    (bind _asbp_first_person_character (cast `/Game/FirstPerson/Blueprints/BP_FirstPersonCharacter` (`self.GetOwner`)))
    (`/Game/Blueprints/Menu/BP_DeathMenuHandler.OpenDeathMenu` (`/Game/FirstPerson/Blueprints/BP_FirstPersonCharacter.DeathMenuHandler` _asbp_first_person_character))))

(event `HealthRegen`
  ;[1 1 1] Health Regeneration
  (`KismetSystemLibrary.RetriggerableDelay` (`self.RegenTime`))
  (bind _output_get (set `self.RegenAmount` (`KismetMathLibrary.FClamp` (* (`self.RegenAmount`) 1.5) -30.0 0.0)))
  (`GameplayStatics.ApplyDamage` (`self.GetOwner`) _output_get))

(event `self.ReceiveBeginPlay`
  (add `Actor.OnTakeAnyDamage` (`self.GetOwner`) (delegate `TakeDamage`)))

(event `TakeDamage`
  (params (DamagedActor :type "Actor Object Reference") (Damage :type "Float (single-precision)") (DamageType :type "DamageType Object Reference") (InstigatedBy :type "Controller Object Reference") (DamageCauser :type "Actor Object Reference"))
  (set `self.OldHealth` (`self.Health`))
  (if (< Damage 0.0)
    (set `self.RegenTime` 1.0)
    (set `self.HitOnce` false)
    (set `self.Health` (`KismetMathLibrary.Conv_IntToDouble` (`KismetMathLibrary.Clamp` (`KismetMathLibrary.FTrunc` (- (`self.Health`) (/ Damage (`self.DefenceLvl`)))) 0 (`KismetMathLibrary.FTrunc` (`self.MaxHealth`)))) :!label _label)
    (elif (>= Damage 50.0)
      (if (<= (- (`self.Health`) Damage) 0.0)
        (set `self.RegenTime` 5.0)
        (set `self.RegenAmount` -1.0)
        (if (== (`self.HitOnce`) true)
          (set `self.Health` 0.0)
          (else
            (set `self.Health` 1.0)
            (set `self.HitOnce` true)))
        (else
          (if (<= (`self.Health`) 50.0) :!label _label_2
            (set `self.DefenceLvl` (+ (`self.DefenceLvl`) 0.1))
            (set `self.MultCount` (`KismetMathLibrary.FClamp` (+ (`self.MultCount`) 1.0) 0.0 5.0))
            (else
              (set `self.DefenceLvl` (`self.PermDefense`))
              (set `self.MultCount` 0.0)))
          (set `self.RegenTime` 5.0)
          (set `self.RegenAmount` -1.0)
          (goto _label)))
      (else
        (goto _label_2))))
  (if (< (`self.Health`) 100.0)
    (`self.HealthRegen`))
  (bind _asbp_first_person_character (cast `/Game/FirstPerson/Blueprints/BP_FirstPersonCharacter` (`self.GetOwner`)))
  (`/Game/Blueprints/HUD/Health/WB_HealthBar.Damage` (`/Game/Blueprints/HUD/HUDLayout.Health` (`/Game/Blueprints/HUD/BP_HUDHandler.HUD` (`/Game/FirstPerson/Blueprints/BP_FirstPersonCharacter.HUDHandler` _asbp_first_person_character))) (- (`self.OldHealth`) (`self.Health`)))
  (`KismetSystemLibrary.PrintString` (`KismetStringLibrary.Conv_DoubleToString` (`self.Health`))))

(event `Key|Three`
  (params (Key :type "Key Structure"))
  (:`Pressed`
    (`GameplayStatics.ApplyDamage` (`self.GetOwner`) 10.0)))