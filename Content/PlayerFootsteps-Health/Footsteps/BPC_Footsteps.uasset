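; Player footstep component that plays surface-specific sounds for walking, running and landing.
; A polling timer checks velocity and MaxWalkSpeed and, along with Left Shift, starts looping walk or run timers that call FootstepTrace.
; Space starts a poll for ground contact that plays FootstepLand and briefly blocks regular steps.
; Both functions sphere-trace downward and pick a cue by physical surface (Snow, Sand, Swamp, Stone), defaulting to Tile.
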(event `self.ReceiveBeginPlay`
  (`self.FootstepTimer`))

(event `JumpLanded`
  ;[1 1 1] Jump code
  (`self.FootstepLand`)
  (set `self.Cooldown` true)
  (`KismetSystemLibrary.Delay` 0.2)
  (set `self.Cooldown` false))

(event `Key|LeftShift`
  (params (Key :type "Key Structure"))
  ;[1 1 1] Sprinting code
  (:`Pressed`
    (set `self.IsRunning` true)
    (`self.FootstepRun`)
    (`KismetSystemLibrary.K2_ClearAndInvalidateTimerHandle` (`self.WalkHandle`)))
  (:`Released`
    (set `self.IsRunning` false)
    (`KismetSystemLibrary.K2_ClearAndInvalidateTimerHandle` (`self.RunHandle`))))

(event `Key|SpaceBar`
  (params (Key :type "Key Structure"))
  ;[1 1 1] Jump code
  (:`Pressed`
    (bind _returnvalue (`KismetSystemLibrary.K2_SetTimerDelegate` (delegate `JumpEnd`) 0.1 true))
    (set `self.JumpHandle` _returnvalue)))

(event `FootstepWalk`
  ;[1 1 1] Walking code
  (`KismetSystemLibrary.K2_SetTimerDelegate` (delegate `Walk`) (`self.Time`) true))

(event `FootstepRun`
  ;[1 1 1] Sprinting code
  (bind _returnvalue (`KismetSystemLibrary.K2_SetTimerDelegate` (delegate `Run`) 0.25 true))
  (set `self.RunHandle` _returnvalue))

(event `JumpEnd`
  ;[1 1 1] Jump code
  (if (`NavMovementComponent.IsMovingOnGround` (`Character.CharacterMovement` (`GameplayStatics.GetPlayerCharacter` 0)))
    (`self.JumpLanded`)
    (`KismetSystemLibrary.K2_ClearAndInvalidateTimerHandle` (`self.JumpHandle`))))

(event `Walk`
  ;[1 1 1] Walking code
  (if (not (`self.IsRunning`))
    (`self.FootstepTrace`)))

(event `Run`
  ;[1 1 1] Sprinting code
  (if (`self.IsRunning`)
    (if (> (`KismetMathLibrary.VSizeXY` (`MovementComponent.Velocity` (`Character.CharacterMovement` (`GameplayStatics.GetPlayerCharacter` 0)))) 0.0)
      (`self.FootstepTrace`))))

(event `FootstepTimer`
  ;[1 1 1] Call FootstepTimer to play
  (`KismetSystemLibrary.K2_SetTimerDelegate` (delegate `FootTime`) 0.01 true))

(event `FootTime`
  ;[1 1 1] Call FootstepTimer to play
  (if (> (`KismetMathLibrary.VSizeXY` (`MovementComponent.Velocity` (`Character.CharacterMovement` (`GameplayStatics.GetPlayerCharacter` 0)))) 0.0)
    (`/Engine/EditorBlueprintResources/StandardMacros.CompareFloat` 600.0 (`CharacterMovementComponent.MaxWalkSpeed` (`Character.CharacterMovement` (`GameplayStatics.GetPlayerCharacter` 0)))
      (:`>`
        (set `self.Time` 0.25)
        (`self.FootstepRun`))
      (:`==`
        (set `self.Time` 0.5)))
    (`KismetSystemLibrary.K2_ClearAndInvalidateTimerHandle` (`self.WalkHandle`))
    (else
      (`self.FootstepWalk`))))

(fn `FootstepLand`
  (bind _returnvalue (`Actor.K2_GetActorLocation` (`self.GetOwner`)))
  (bind _capsulecomponent (`Character.CapsuleComponent` (`GameplayStatics.GetPlayerCharacter` 0)))
  (bind (_outhit _returnvalue_2) (`KismetSystemLibrary.SphereTraceSingle` _returnvalue (`KismetMathLibrary.MakeVector` (.x _returnvalue) (.y _returnvalue) (- (.z _returnvalue) (`CapsuleComponent.GetScaledCapsuleHalfHeight` _capsulecomponent))) (`CapsuleComponent.GetScaledCapsuleRadius` _capsulecomponent) "TraceTypeQuery1"))
  (if _returnvalue_2
    (set `self.HitLocation` (`.Location` (`GameplayStatics.BreakHitResult` _outhit)))
    (switch `EPhysicalSurface` (`GameplayStatics.GetSurfaceType` _outhit)
      (:`SurfaceType_Default`
        (`GameplayStatics.PlaySoundAtLocation` "/Game/SoundEffects/Cues/Steps/TileSteps_Cue.TileSteps_Cue" (`self.HitLocation`) (struct) 1.0 1.0 0.0 null null null null :!label _label))
      (:`SurfaceType1`
        (`GameplayStatics.PlaySoundAtLocation` "/Game/SoundEffects/Cues/Steps/SnowSteps_Cue.SnowSteps_Cue" (`self.HitLocation`) (struct) 1.0 1.0 0.0 null null null null))
      (:`SurfaceType2`
        (`GameplayStatics.PlaySoundAtLocation` "/Game/SoundEffects/Cues/Steps/SandSteps_Cue.SandSteps_Cue" (`self.HitLocation`) (struct) 1.0 1.0 0.0 null null null null))
      (:`SurfaceType3`
        (`GameplayStatics.PlaySoundAtLocation` "/Game/SoundEffects/Cues/Steps/SwampSteps_Cue.SwampSteps_Cue" (`self.HitLocation`) (struct) 1.0 1.0 0.0 null null null null))
      (:`SurfaceType4`
        (`GameplayStatics.PlaySoundAtLocation` "/Game/SoundEffects/Cues/Steps/StoneSteps_Cue.StoneSteps_Cue" (`self.HitLocation`) (struct) 1.0 1.0 0.0 null null null null))
      (:`SurfaceType5`
        (goto _label)))))

(fn `FootstepTrace`
  (bind _returnvalue (`Actor.K2_GetActorLocation` (`self.GetOwner`)))
  (bind _capsulecomponent (`Character.CapsuleComponent` (`GameplayStatics.GetPlayerCharacter` 0)))
  (if (not (`self.Cooldown`))
    (bind (_outhit _returnvalue_2) (`KismetSystemLibrary.SphereTraceSingle` _returnvalue (`KismetMathLibrary.MakeVector` (.x _returnvalue) (.y _returnvalue) (- (.z _returnvalue) (`CapsuleComponent.GetScaledCapsuleHalfHeight` _capsulecomponent))) (`CapsuleComponent.GetScaledCapsuleRadius` _capsulecomponent) "TraceTypeQuery1"))
    (if _returnvalue_2
      (set `self.HitLocation` (`.Location` (`GameplayStatics.BreakHitResult` _outhit)))
      (switch `EPhysicalSurface` (`GameplayStatics.GetSurfaceType` _outhit)
        (:`SurfaceType_Default`
          (`GameplayStatics.PlaySoundAtLocation` "/Game/SoundEffects/Cues/Steps/TileSteps_Cue.TileSteps_Cue" (`self.HitLocation`) (struct) 1.0 1.0 0.0 null null null null :!label _label))
        (:`SurfaceType1`
          (`GameplayStatics.PlaySoundAtLocation` "/Game/SoundEffects/Cues/Steps/SnowSteps_Cue.SnowSteps_Cue" (`self.HitLocation`) (struct) 1.0 1.0 0.0 null null null null))
        (:`SurfaceType2`
          (`GameplayStatics.PlaySoundAtLocation` "/Game/SoundEffects/Cues/Steps/SandSteps_Cue.SandSteps_Cue" (`self.HitLocation`) (struct) 1.0 1.0 0.0 null null null null))
        (:`SurfaceType3`
          (`GameplayStatics.PlaySoundAtLocation` "/Game/SoundEffects/Cues/Steps/SwampSteps_Cue.SwampSteps_Cue" (`self.HitLocation`) (struct) 1.0 1.0 0.0 null null null null))
        (:`SurfaceType4`
          (`GameplayStatics.PlaySoundAtLocation` "/Game/SoundEffects/Cues/Steps/StoneSteps_Cue.StoneSteps_Cue" (`self.HitLocation`) (struct) 1.0 1.0 0.0 null null null null))
        (:`SurfaceType5`
          (goto _label))))))