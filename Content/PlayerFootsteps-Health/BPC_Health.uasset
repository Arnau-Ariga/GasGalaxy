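; Health component that handles damage, adaptive defense, one-shot protection and automatic regeneration for its owner.
; Damage is divided by a defense level that climbs with hits at low health.
; A heavy lethal hit first leaves 1 health, killing only if repeated before healing.
; Regeneration uses a retriggerable delay, feeding growing negative damage through ApplyDamage to loop while health is below 100.
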(event `TakeDamage`
  (params (Damage :type "Float (single-precision)") (DamageType :type "DamageType Object Reference") (InstigatedBy :type "Controller Object Reference") (DamageCauser :type "Actor Object Reference"))
  (if (< Damage 0.0)
    (set `self.RegenTime` 1.0)
    (set `self.HitOnce` false)
    (set `self.Health` (`KismetMathLibrary.Conv_IntToDouble` (`KismetMathLibrary.Clamp` (`KismetMathLibrary.FTrunc` (- (`self.Health`) (/ Damage (`self.DefenceLvl`)))) 0 (`KismetMathLibrary.FTrunc` (`self.MaxHealth`)))) :!label _label)
    (elif (>= Damage 50.0)
      (if (<= (- (`self.Health`) Damage) 0.0)
        (set `self.RegenTime` 5.0)
        (set `self.RegenAmount` -1.0)
        (if (== (`self.HitOnce`) true)
          (set `self.Health` 0.0)
          (else
            (set `self.Health` 1.0)
            (set `self.HitOnce` true)))
        (else
          (if (<= (`self.Health`) 50.0) :!label _label_2
            (set `self.DefenceLvl` (+ (`self.DefenceLvl`) 0.1))
            (set `self.MultCount` (`KismetMathLibrary.FClamp` (+ (`self.MultCount`) 1.0) 0.0 5.0))
            (else
              (set `self.DefenceLvl` (`self.PermDefense`))
              (set `self.MultCount` 0.0)))
          (set `self.RegenTime` 5.0)
          (set `self.RegenAmount` -1.0)
          (goto _label)))
      (else
        (goto _label_2))))
  (if (< (`self.Health`) 100.0)
    (`self.HealthRegen`))
  (`KismetSystemLibrary.PrintString` (`KismetStringLibrary.Conv_DoubleToString` (`self.Health`))))

(event `HealthRegen`
  ;[1 1 1] Health Regeneration
  (`KismetSystemLibrary.RetriggerableDelay` (`self.RegenTime`))
  (bind _output_get (set `self.RegenAmount` (`KismetMathLibrary.FClamp` (* (`self.RegenAmount`) 1.5) -30.0 0.0)))
  (`GameplayStatics.ApplyDamage` (`self.GetOwner`) _output_get)
  (`KismetSystemLibrary.PrintString` "Hello"))