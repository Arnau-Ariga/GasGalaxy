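; BP_Chest is an interactable chest that consumes a key from the inventory to give out a random equipment module.
; On interaction with a key, it marks itself opened, spawns a BP_PickupableModule with a random module name at the ModuleSpawn point, and destroys its trigger.
; Without a key it shows a "Need A Key" pop-up.
; It supplies an "Open Chest" prompt and stops being interactable once opened.
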(event `/Game/Blueprints/Interact/BPI_Interactable.Interact`
  (bind _wasremoved (`/Game/Blueprints/Inventory/FL_InventoryFunctions.RemoveKeyItemFromInventory` "Key"))
  (if _wasremoved
    (set `self.IsOpened` true)
    (`|SpawnActorFromClass` "/Game/Blueprints/Equipment/Module/BP_PickupableModule.BP_PickupableModule_C" (`KismetMathLibrary.Conv_VectorToTransform` (`SceneComponent.K2_GetComponentLocation` (`self.ModuleSpawn`))) "Undefined" "MultiplyWithRoot" null (`/Game/Blueprints/Equipment/Module/FL_ModuleFunctions.GetRandomModuleName`) null)
    (`ActorComponent.K2_DestroyComponent` (`self.Trigger`))
    (else
      (`/Game/Blueprints/PopUp/FL_PopUpFunctions.SendPopUp` "/Game/Textures/Images/Icons/WhiteKeyIcon.WhiteKeyIcon" "Need A Key"))))

(fn `GetPrompt`
  (returns (Prompt :type String))
  (return "Open Chest"))

(fn `IsInteractable`
  (returns (IsInteractable :type Boolean))
  (return (not (`self.IsOpened`))))

(fn `UserConstructionScript`)