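; BP_PickupableModule is a world pickup for an equipment module, identified by its ModuleName.
; On BeginPlay it fills two W_ModuleImage widgets, one with the module's image and one with a white icon chosen by indexing an array with the module type.
; GetPrompt builds the "Pick Up" text from the module name, and PickUp adds the module to the inventory and returns that call's result.
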(event `self.ReceiveBeginPlay`
  ;[1 1 1] Set Module Images
  (bind _asw_module_image (cast `/Game/Blueprints/Equipment/Module/W_ModuleImage` (`WidgetComponent.GetWidget` (`self.ModuleImage`))))
  (`/Game/Blueprints/Equipment/Module/W_ModuleImage.SetModuleImage` _asw_module_image (`/Game/Blueprints/Equipment/Module/FL_ModuleFunctions.GetModuleImage` (`self.ModuleName`)))
  ;[1 1 1] Set Module Type Image
  (bind _asw_module_image_2 (cast `/Game/Blueprints/Equipment/Module/W_ModuleImage` (`WidgetComponent.GetWidget` (`self.ModuleTypeImage`))))
  (`/Game/Blueprints/Equipment/Module/W_ModuleImage.SetModuleImage` _asw_module_image_2 (`|GetArrayItem` (`|MakeArray` "/Game/Textures/Images/Icons/WhiteShirtIcon.WhiteShirtIcon" "/Game/Textures/Images/Icons/WhiteBootsIcon.WhiteBootsIcon" "/Game/Textures/Images/Icons/WhiteRifleIcon.WhiteRifleIcon" "/Game/Textures/Images/Icons/WhiteSwordIcon.WhiteSwordIcon" "/Game/Textures/Images/Icons/WhiteGearIcon.WhiteGearIcon" :!type "Texture2D Object Reference") (`KismetMathLibrary.Conv_ByteToInt` (`/Game/Blueprints/Equipment/Module/FL_ModuleFunctions.GetModuleType` (`self.ModuleName`))))))

(fn `GetPrompt`
  (returns (Prompt :type String))
  (return (`KismetStringLibrary.Concat_StrStr` "Pick Up " (`KismetStringLibrary.Conv_NameToString` (`self.ModuleName`)) " Module")))

(fn `PickUp`
  (returns (PickedUp :type Boolean))
  (bind _moduleadded (`/Game/Blueprints/Inventory/FL_InventoryFunctions.AddModuleToInventory` (`self.ModuleName`)))
  (return _moduleadded))

(fn `UserConstructionScript`)