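; Base component for first-person equipment, with empty use and release events that fire from Enhanced Input actions.
; On BeginPlay it attaches to a socket on the owning character's first-person mesh, adds the equipment mapping context and sets the AnimBP holding pose.
; Unequip destroys the component, resets the pose and removes the mapping context.
; GetProperty looks up a named value, falling back to a default, then adds each equipment module's contribution.
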(event `self.ReceiveBeginPlay`
  (bind _asbp_first_person_character (cast `/Game/FirstPerson/Blueprints/BP_FirstPersonCharacter` (`self.GetOwner`)))
  (bind _output_get (set `self.First PersonCharacter` _asbp_first_person_character))
  ;[1 1 1] Add Component To Skeletal Mesh
  (`self.K2_AttachToComponent` (`/Game/FirstPerson/Blueprints/BP_FirstPersonCharacter.FirstPersonMesh` _output_get) (`self.SocketName`) "SnapToTarget" "SnapToTarget" "SnapToTarget")
  ;[1 1 1] Add Action Map
  (bind _asplayer_controller (cast `PlayerController` (`Pawn.GetController` (`self.First PersonCharacter`))))
  (bind _returnvalue (pcsubsystem `EnhancedInputLocalPlayerSubsystem` _asplayer_controller))
  (`/Engine/EditorBlueprintResources/StandardMacros.IsValid` _returnvalue
    (:`Is Valid`
      (`EnhancedInputSubsystemInterface.AddMappingContext` _returnvalue "/Game/Blueprints/Equipment/Input/IMC_Equipment.IMC_Equipment" 1 (struct))
      ;[1 1 1] Update Anim Instance
      (bind _asfirst_person_anim_bp (cast `/Game/FirstPersonArms/Animations/FirstPerson_AnimBP` (`self.GetAnimInstance` (`/Game/FirstPerson/Blueprints/BP_FirstPersonCharacter.FirstPersonMesh` (`self.First PersonCharacter`)))))
      (set `/Game/FirstPersonArms/Animations/FirstPerson_AnimBP.HoldingPose` (`self.EquipmentPose`) _asfirst_person_anim_bp))))

(event `Unequip`
  ;[1 1 1] Try To Destroy Component
  (if (not (`self.IsBeingDestroyed`))
    (`self.K2_DestroyComponent`))
  ;[1 1 1] Set Holding Pose To None
  (bind _asfirst_person_anim_bp (cast `/Game/FirstPersonArms/Animations/FirstPerson_AnimBP` (`self.GetAnimInstance` (`/Game/FirstPerson/Blueprints/BP_FirstPersonCharacter.FirstPersonMesh` (`self.First PersonCharacter`)))))
  (set `/Game/FirstPersonArms/Animations/FirstPerson_AnimBP.HoldingPose` "NewEnumerator3" _asfirst_person_anim_bp)
  ;[1 1 1] Remove Action Map
  (bind _asplayer_controller (cast `PlayerController` (`Pawn.GetController` (`self.First PersonCharacter`))))
  (bind _returnvalue (pcsubsystem `EnhancedInputLocalPlayerSubsystem` _asplayer_controller))
  (`/Engine/EditorBlueprintResources/StandardMacros.IsValid` _returnvalue
    (:`Is Valid`
      (`EnhancedInputSubsystemInterface.RemoveMappingContext` _returnvalue "/Game/Blueprints/Equipment/Input/IMC_Equipment.IMC_Equipment" (struct)))))

(event `EnhancedInput|/Game/Blueprints/Equipment/Input/IA_UseItem`
  (params (ActionValue :type Boolean) (ElapsedSeconds :type "Float (double-precision)") (TriggeredSeconds :type "Float (double-precision)") (InputAction :type "InputAction Object Reference" :default "/Game/Blueprints/Equipment/Input/IA_UseItem.IA_UseItem"))
  ;[1 1 1] Equipment Actions
  (:`Triggered`
    (`self.OnUseItem`)))

(event `EnhancedInput|/Game/Blueprints/Equipment/Input/IA_ReleaseItem`
  (params (ActionValue :type Boolean) (ElapsedSeconds :type "Float (double-precision)") (TriggeredSeconds :type "Float (double-precision)") (InputAction :type "InputAction Object Reference" :default "/Game/Blueprints/Equipment/Input/IA_ReleaseItem.IA_ReleaseItem"))
  ;[1 1 1] Equipment Actions
  (:`Triggered`
    (`self.OnReleaseItem`)))

(event `OnUseItem`
  ;[1 1 1] Equipment Actions
)

(event `OnReleaseItem`
  ;[1 1 1] Equipment Actions
)

(fn `GetProperty`
  (params (PropertyName :type Name) (DefaultValue :type "Float (double-precision)"))
  (returns (Value :type "Float (double-precision)"))
  (locals (PropertyValue :type "Float (double-precision)") (valueHasOverride :type Boolean))
  (bind (_value _returnvalue) (`BlueprintMapLibrary.Map_Find` (`self.EquipmentProperties`) PropertyName))
  (if _returnvalue
    (set `local.PropertyValue` _value)
    (else
      (set `local.PropertyValue` DefaultValue)))
  (for _array_element (`/Game/Blueprints/Inventory/Item/BP_ItemInstance.Modules` (`/Game/Blueprints/Inventory/FL_InventoryFunctions.GetItemFromInventory` (`/Game/Blueprints/Inventory/BP_Inventory.EquippedItemSlotIndex` (`/Game/Blueprints/Inventory/FL_InventoryFunctions.GetInventory`))))
    (set `local.PropertyValue` (+ (`local.PropertyValue`) (`BlueprintMapLibrary.Map_Find` (`/Game/Blueprints/Equipment/Module/FL_ModuleFunctions.GetModuleProperties` _array_element) PropertyName))))
  (return (`local.PropertyValue`)))