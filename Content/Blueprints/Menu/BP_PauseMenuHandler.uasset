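; BP_PauseMenuHandler opens the pause menu when the player triggers the pause input.
; On BeginPlay it creates and stores a W_PauseMenu widget and adds the IMC_PauseMenu Enhanced Input mapping context to the first player controller.
; IA_PauseGame adds that widget to the viewport, switches to focused UI-only input, shows the cursor and pauses the game.
; It contains no closing or unpause logic.
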(event `self.ReceiveBeginPlay`
  (bind _returnvalue (pcsubsystem `EnhancedInputLocalPlayerSubsystem` (`GameplayStatics.GetPlayerController` 0)))
  (`|ExecutionSequence`
    (:`then_0`
      ;[1 1 1] Create Pause Menu Widget
      (bind _returnvalue_2 (`|CreateWidget` "/Game/Blueprints/Menu/W_PauseMenu.W_PauseMenu_C" (`GameplayStatics.GetPlayerController` 0)))
      (set `self.PauseMenu` _returnvalue_2))
    (:`then_1`
      ;[1 1 1] Add Pause Menu Mapping Context To Player Controller
      (`/Engine/EditorBlueprintResources/StandardMacros.IsValid` _returnvalue
        (:`Is Valid`
          (`EnhancedInputSubsystemInterface.AddMappingContext` _returnvalue "/Game/Blueprints/Menu/Input/IMC_PauseMenu.IMC_PauseMenu" 1 (struct)))))))

(event `EnhancedInput|/Game/Blueprints/Menu/Input/IA_PauseGame`
  (params (ActionValue :type Boolean) (ElapsedSeconds :type "Float (double-precision)") (TriggeredSeconds :type "Float (double-precision)") (InputAction :type "InputAction Object Reference" :default "/Game/Blueprints/Menu/Input/IA_PauseGame.IA_PauseGame"))
  (bind _returnvalue (`GameplayStatics.GetPlayerController` 0))
  (bind _pausemenu (`self.PauseMenu`))
  ;[1 1 1] Open Pause Menu
  (:`Triggered`
    (`UserWidget.AddToViewport` _pausemenu 0)
    (`WidgetBlueprintLibrary.SetInputMode_UIOnlyEx` _returnvalue _pausemenu)
    (set `PlayerController.bShowMouseCursor` true _returnvalue)
    (`GameplayStatics.SetGamePaused` true)))