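; Interaction component for the first-person character that lets the player use objects implementing BPI_Interactable.
; Each tick it picks the first interactable actor overlapping the owner's capsule, then confirms it with a short camera line trace.
; While that target is looked at, it shows a prompt widget with the target's custom text or a default.
; It adds its own Enhanced Input context on BeginPlay, and the Interact action calls Interact on the target.
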(event `self.ReceiveBeginPlay`
  ;[1 1 1] Add Interact Input Mapping Context To Player Controller
  (`EnhancedInputSubsystemInterface.AddMappingContext` (pcsubsystem `EnhancedInputLocalPlayerSubsystem` (`GameplayStatics.GetPlayerController` 0)) "/Game/Blueprints/Interact/Input/IMC_Interact.IMC_Interact" 1 (struct)))

(event `self.ReceiveTick`
  (params (DeltaSeconds :type "Float (single-precision)"))
  (`|ExecutionSequence`
    (:`then_0`
      (`self.FindInteractable`))
    (:`then_1`
      (`self.RaycastToInteractable`))
    (:`then_2`
      (`self.DisplayInteractPrompt`))))

(event `FindInteractable`
  ;[1 1 1] Find Interactable
  (set `self.Interactable` null)
  (bind _asbp_first_person_character (cast `/Game/FirstPerson/Blueprints/BP_FirstPersonCharacter` (`self.GetOwner`)))
  (for _array_element (`PrimitiveComponent.GetOverlappingActors` (`Character.CapsuleComponent` _asbp_first_person_character) null)
    (bind _asbpi_interactable (cast `/Game/Blueprints/Interact/BPI_Interactable` _array_element))
    (bind _isinteractable (`/Game/Blueprints/Interact/BPI_Interactable.IsInteractable` _asbpi_interactable))
    (if _isinteractable
      (set `self.Interactable` _asbpi_interactable)
      (break))))

(event `RaycastToInteractable`
  ;[1 1 1] Raycast To Interactable
  (set `self.LookingAtInteractable` false)
  (if (`KismetSystemLibrary.IsValidInterface` (`self.Interactable`))
    (bind _asbp_first_person_character (cast `/Game/FirstPerson/Blueprints/BP_FirstPersonCharacter` (`self.GetOwner`)))
    (bind _firstpersoncamera (`/Game/FirstPerson/Blueprints/BP_FirstPersonCharacter.FirstPersonCamera` _asbp_first_person_character))
    (bind _returnvalue (`SceneComponent.K2_GetComponentLocation` _firstpersoncamera))
    (bind _outhit (`KismetSystemLibrary.LineTraceSingle` _returnvalue (+ _returnvalue (* (`KismetMathLibrary.GetForwardVector` (`SceneComponent.K2_GetComponentRotation` _firstpersoncamera)) 100.0)) "TraceTypeQuery1"))
    (bind (_bblockinghit _binitialoverlap _time _distance _location _impactpoint _normal _impactnormal _physmat _hitactor) (`GameplayStatics.BreakHitResult` _outhit))
    (cast `/Game/Blueprints/Interact/BPI_Interactable` _hitactor)
    (set `self.LookingAtInteractable` (== _hitactor (`self.Interactable`)))))

(event `DisplayInteractPrompt`
  (bind _returnvalue (`KismetSystemLibrary.IsValid` (`self.InteractPrompt`)))
  ;[1 1 1] Display Interact Prompt
  (if (`self.LookingAtInteractable`)
    (if (not _returnvalue)
      (bind _returnvalue_2 (`|CreateWidget` "/Game/Blueprints/Interact/W_InteractPrompt.W_InteractPrompt_C" (`GameplayStatics.GetPlayerController` 0)))
      (bind _output_get (set `self.InteractPrompt` _returnvalue_2))
      (`UserWidget.AddToViewport` _output_get 0)
      (bind _prompt (`/Game/Blueprints/Interact/BPI_Interactable.GetPrompt` (`self.Interactable`)))
      (if (`KismetStringLibrary.IsEmpty` _prompt)
        (`/Game/Blueprints/Interact/W_InteractPrompt.SetPrompt` _output_get "Interact")
        (else
          (`/Game/Blueprints/Interact/W_InteractPrompt.SetPrompt` _output_get _prompt))))
    (elif _returnvalue
      (`Widget.RemoveFromParent` (`self.InteractPrompt`))
      (set `self.InteractPrompt` null))))

(event `EnhancedInput|/Game/Blueprints/Interact/Input/IA_Interact`
  (params (ActionValue :type Boolean) (ElapsedSeconds :type "Float (double-precision)") (TriggeredSeconds :type "Float (double-precision)") (InputAction :type "InputAction Object Reference" :default "/Game/Blueprints/Interact/Input/IA_Interact.IA_Interact"))
  ;[1 1 1] Interact With Interactable
  (:`Triggered`
    (if (`self.LookingAtInteractable`)
      (`/Game/Blueprints/Interact/BPI_Interactable.Interact` (`self.Interactable`)))))