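; BP_NPC is an interactable talking NPC that offers a "Talk" prompt and steps through an array of dialog lines.
; Interact creates or reuses a W_Dialog widget, then IncrementIndexHelper shows the current line, prints its emotion and advances until the last entry.
; The player leaving the sphere removes the widget without resetting the index.
; A placeholder-substitution helper exists but is uncalled here; quest handling appears only in comments.
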(event `CreateWidget`
  ;[1 1 1] Create the widget whenever they talk
  (`self.InstructionWidget`
    (:`then`
      _)
    (:`else`
      (bind _returnvalue (`|CreateWidget` "/Game/Blueprints/NPC/W_Dialog.W_Dialog_C"))
      (set `self.InstructionWidget` _returnvalue)))
  (`UserWidget.AddToViewport` (`self.InstructionWidget`) 0)
  (set `self.IsTalking` true))

(event `self.Sphere.OnComponentEndOverlap`
  (params (OverlappedComponent :type "PrimitiveComponent Object Reference") (OtherActor :type "Actor Object Reference") (OtherComp :type "PrimitiveComponent Object Reference") (OtherBodyIndex :type Integer))
  ;[1 1 1] Remove Prompt From Viewport if Out Range
  (cast `/Game/FirstPerson/Blueprints/BP_FirstPersonCharacter` OtherActor)
  (bind _instructionwidget (`self.InstructionWidget`)
    (:`then`
      (if (`Widget.IsInViewport` _instructionwidget)
        (`Widget.RemoveFromParent` (`self.InstructionWidget`))
        (set `self.IsTalking` false)))
    (:`else`)))

(event `/Game/Blueprints/Interact/BPI_Interactable.Interact`
  ;[1 1 1] Increment the index for the dialog and Assign a Quest (if QuestGiver)
  (if (`self.IsTalking`)
    (`self.IncrementIndex`)
    (else
      (`self.CreateWidget`)
      (`self.IncrementIndex`)))
  (set `self.IsTalking` true))

(event `IncrementIndex`
  ;[1 1 1] Increment the index for the dialog and Assign a Quest or Complete a quest (if QuestGiver)
  (`self.Increment Index Helper` (`self.Dialog`)))

(fn `GetPrompt`
  (returns (Prompt :type String))
  (return "Talk"))

(fn `Increment Index Helper`
  (params (Array :type "Array of /Game/Blueprints/NPC/DialogLine Structure"))
  (returns (IsAtEnd :type Boolean))
  (bind _dialogindex (`self.DialogIndex`))
  (bind (_dialogline _emotionofline) (break `/Game/Blueprints/NPC/DialogLine` (`|GetArrayItem` Array _dialogindex)))
  ;[1 1 1] Goes Through Array and Changes Widget
  (bind _instructionwidget (`self.InstructionWidget`)
    (:`then`
      (set `/Game/Blueprints/NPC/W_Dialog.Dialog` _dialogline _instructionwidget)
      (`KismetSystemLibrary.PrintString` (`|GetEnumeratorNameAsString` _emotionofline))
      (if (< _dialogindex (`KismetArrayLibrary.Array_LastIndex` Array))
        (bind _result (`/Engine/EditorBlueprintResources/StandardMacros.IncrementInt` _dialogindex)
          (:`  `
            (set `self.DialogIndex` _result)))
        (else
          (return true))))
    (:`else`)))

(fn `IsInteractable`
  (returns (IsInteractable :type Boolean))
  (return true))

(fn `ReplaceWithArray`
  (params (StringArray :type "Array of String") (QuestData :type String))
  ;[1 1 1] Replace every "%" in the array with the replacer variable
  (for (_array_element _array_index) StringArray
    (`KismetArrayLibrary.Array_Set` StringArray _array_index (`KismetStringLibrary.Replace` _array_element "%" QuestData))
    (break)))

(fn `UserConstructionScript`)