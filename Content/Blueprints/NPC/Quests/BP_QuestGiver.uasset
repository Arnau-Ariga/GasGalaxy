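; Quest-giver NPC that assigns a random quest (simple fetch or kill enemies), registers it with the player and runs its dialog.
; Dialog comes from a random data table row with "%" placeholders substituted, then advances through before, during and after stages.
; Fetch quests spawn a key item and activate at BeginPlay.
; Tick polls inventory and completion to switch to post-quest dialog, whose end calls a placeholder reward.
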(event `self.ReceiveBeginPlay`
  ;[1 1 1] Comment
  (`self.Construct Quest`)
  (switch `/Game/Blueprints/NPC/Quests/E_QuestType` (`self.QuestType`)
    (:`NewEnumerator0`
      (set `/Game/Blueprints/NPC/Quests/BP_Quest.IsQuestActive` true (`self.Quest`))
      (bind _returnvalue (`|SpawnActorFromClass` "/Game/Blueprints/Inventory/KeyItem/BP_PickupableKeyItem.BP_PickupableKeyItem_C" (`KismetMathLibrary.MakeTransform` (`KismetMathLibrary.MakeVector` (`KismetMathLibrary.RandomFloatInRange` 900.0 1100.0) (`KismetMathLibrary.RandomFloatInRange` 900.0 1100.0) 150.0)) "Undefined" "MultiplyWithRoot" null "Diamond" (`GameplayStatics.GetPlayerPawn` 0)))
      (set `self.KeyItem` _returnvalue)
      (bind _asbp_simple_fetch_quest (cast `/Game/Blueprints/NPC/Quests/BP_SimpleFetchQuest` (`self.Quest`)))
      (set `/Game/Blueprints/NPC/Quests/BP_SimpleFetchQuest.KeyItemName` (`/Game/Blueprints/Inventory/KeyItem/BP_PickupableKeyItem.KeyItemName` _returnvalue) _asbp_simple_fetch_quest))))

(event `Modify Dialog`
  (params (Dialog :type "/Game/Blueprints/NPC/Quests/S_Dialog Structure"))
  ;[1 1 1] Replaces the % in the Dialog Struct
  (bind _output_get (set `self.QuestDialog` Dialog))
  (bind (_initialdialog _duringquestdialog _postquestdialog) (break `/Game/Blueprints/NPC/Quests/S_Dialog` _output_get))
  (bind _newarray (`self.ReplaceArray` _initialdialog (`self.QuestData`)))
  (set `self.IntroDialog` _newarray)
  (bind _newarray_2 (`self.ReplaceArray` _duringquestdialog (`self.QuestData`)))
  (set `self.MidDialog` _newarray_2)
  (bind _newarray_3 (`self.ReplaceArray` _postquestdialog (`self.QuestData`)))
  (set `self.PostDialog` _newarray_3))

(event `self.IncrementIndex`
  ;[1 1 1] IncrementIndex for QuestNPC
  (switch `/Game/Blueprints/NPC/Quests/E_QuestProgress` (`self.QuestProgress`)
    (:`NewEnumerator0`
      (bind _isatend (`self.Increment Index Helper` (`self.IntroDialog`)))
      (if _isatend
        (set `self.QuestProgress` "NewEnumerator1")
        (set `self.DialogIndex` 0)
        (set `/Game/Blueprints/NPC/Quests/BP_Quest.IsQuestActive` true (`self.Quest`))
        (bind _returnvalue (`|CreateWidget` "/Game/Blueprints/NPC/Quests/W_Notification.W_Notification_C"))
        (`UserWidget.AddToViewport` _returnvalue 0)))
    (:`NewEnumerator1`
      (`self.Increment Index Helper` (`self.MidDialog`)))
    (:`NewEnumerator2`
      (bind _isatend_2 (`self.Increment Index Helper` (`self.PostDialog`)))
      (if _isatend_2
        (`self.Reward Player`)))))

(event `Add Dialog`
  ;[1 1 1] Adds A Dialog for a Quest Giver Based on its QuestType
  (switch `/Game/Blueprints/NPC/Quests/E_QuestType` (`self.QuestType`)
    (:`NewEnumerator0`
      (bind _randomrow (`self.Get Random Data Table Row` "/Game/Blueprints/NPC/Quests/DT_SimpleFetchQuestTable.DT_SimpleFetchQuestTable"))
      (`self.Modify Dialog` _randomrow))
    (:`NewEnumerator1`
      (bind _randomrow_2 (`self.Get Random Data Table Row` "/Game/Blueprints/NPC/Quests/DT_KillXEnemiesTable.DT_KillXEnemiesTable"))
      (`self.Modify Dialog` _randomrow_2))))

(event `Reward Player`
  ;[1 1 1] Reward the player when they are done with a quest
  (if (not (`self.HasRewarded`))
    (`KismetSystemLibrary.PrintString` "TODO: REWARD PLAYER")
    (set `self.HasRewarded` true)))

(event `AddToQuestList`
  (params (Quest :type "/Game/Blueprints/NPC/Quests/BP_Quest Object Reference"))
  ;[1 1 1] Adds a Quest to the QuestList in the Player
  (bind _asbp_first_person_character (cast `/Game/FirstPerson/Blueprints/BP_FirstPersonCharacter` (`GameplayStatics.GetPlayerPawn` 0)))
  (`KismetArrayLibrary.Array_Add` (`/Game/Blueprints/NPC/Quests/BP_QuestList.Quests` (`/Game/FirstPerson/Blueprints/BP_FirstPersonCharacter.BP_QuestList` _asbp_first_person_character)) Quest)
  (set `self.Quest` Quest))

(event `Construct Quest`
  ;[1 1 1] Make a Quest
  (bind _output_get (set `self.QuestType` (cast `/Game/Blueprints/NPC/Quests/E_QuestType` (`self.GetRandomQuestType`))))
  (switch `/Game/Blueprints/NPC/Quests/E_QuestType` _output_get
    (:`NewEnumerator0`
      (bind _returnvalue (`|GenericCreateObject` "/Game/Blueprints/NPC/Quests/BP_SimpleFetchQuest.BP_SimpleFetchQuest_C" self))
      (`self.AddToQuestList` _returnvalue)
      (set `self.QuestData` "11/7")
      (`self.Add Dialog`))
    (:`NewEnumerator1`
      (bind _returnvalue_2 (`|GenericCreateObject` "/Game/Blueprints/NPC/Quests/BP_KillXEnemiesQuest.BP_KillXEnemiesQuest_C" self))
      (`self.AddToQuestList` _returnvalue_2)
      (set `self.QuestData` "penguins")
      (`self.Add Dialog`))))

(event `self.ReceiveTick`
  (params (DeltaSeconds :type "Float (single-precision)"))
  (bind _quest (`self.Quest`))
  ;[1 1 1] Checks if the Quest is Done Every Tick
  (`parent.ReceiveTick` 0.0)
  (`self.CheckInventory`)
  (`/Game/Blueprints/NPC/Quests/BP_Quest.CheckQuestCompletion` _quest)
  (if (and (`/Game/Blueprints/NPC/Quests/BP_Quest.IsQuestComplete` _quest) (== (`self.QuestProgress`) (`KismetSystemLibrary.MakeLiteralByte` (enumliteral `/Game/Blueprints/NPC/Quests/E_QuestProgress` "NewEnumerator1"))))
    (set `self.DialogIndex` 0)
    (set `self.QuestProgress` "NewEnumerator2")
    (`/Game/Blueprints/Inventory/FL_InventoryFunctions.RemoveKeyItemFromInventory` "Diamond")))

(fn `CheckInventory`
  ;[1 1 1] Checks if the inventory containsthe key item
  (switch `/Game/Blueprints/NPC/Quests/E_QuestType` (`self.QuestType`)
    (:`NewEnumerator0`
      (bind _asbp_simple_fetch_quest (cast `/Game/Blueprints/NPC/Quests/BP_SimpleFetchQuest` (`self.Quest`)))
      (set `/Game/Blueprints/NPC/Quests/BP_SimpleFetchQuest.HasFoundItem` (> (`/Game/Blueprints/Inventory/FL_InventoryFunctions.GetKeyItemCountFromInventory` (`/Game/Blueprints/NPC/Quests/BP_SimpleFetchQuest.KeyItemName` _asbp_simple_fetch_quest)) 0) _asbp_simple_fetch_quest))))

(fn `Get Random Data Table Row`
  (params (DataTable :type "DataTable Object Reference"))
  (returns (RandomRow :type "/Game/Blueprints/NPC/Quests/S_Dialog Structure"))
  (`/Engine/EditorBlueprintResources/StandardMacros.IsValid` DataTable
    (:`Is Valid`
      (bind _outrownames (`DataTableFunctionLibrary.GetDataTableRowNames` DataTable))
      (bind _returnvalue (`|GetDataTableRow` DataTable (`KismetArrayLibrary.Array_Random` _outrownames))
        (:`then`
          (return _returnvalue))))))

(fn `GetRandomQuestType`
  (returns (RandomQuestType :type Byte))
  (return (cast `/Game/Blueprints/NPC/Quests/E_QuestType` (`KismetMathLibrary.Conv_IntToByte` (`KismetMathLibrary.RandomIntegerInRange` 0 (- (enumcount `/Game/Blueprints/NPC/Quests/E_QuestType`) 1))))))

(fn `ReplaceArray`
  (params (InputArray :type "Array of /Game/Blueprints/NPC/S_DialogLine Structure") (QuestData :type String))
  (returns (NewArray :type "Array of /Game/Blueprints/NPC/S_DialogLine Structure"))
  ;[1 1 1] Replace every "%" in the array with the replacer variable
  (for (_array_element _array_index) InputArray
    (bind (_dialogline _emotionofline) (break `/Game/Blueprints/NPC/S_DialogLine` _array_element))
    (`KismetArrayLibrary.Array_Set` InputArray _array_index (make `/Game/Blueprints/NPC/S_DialogLine` (`KismetStringLibrary.Replace` _dialogline "%" QuestData) _emotionofline)))
  (return (`local.InputArray`)))

(fn `UserConstructionScript`
  (`parent.UserConstructionScript`))