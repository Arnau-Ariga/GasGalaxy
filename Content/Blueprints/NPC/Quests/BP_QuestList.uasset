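; BP_QuestList is a quest list, owned by the first-person player character, that tracks kill-count progress.
; EliminateEnemy loops through Quests to increment a BP_KillXEnemiesQuest's kill count and check completion, breaking after the first one updated.
; The enemy name is not yet checked, as the logic is placeholder.
; A debug P key marks every active quest complete to test NPC state changes.
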(event `EliminateEnemy`
  (params (Name :type String))
  ;[1 1 1] Somewhat placeholder code for now. Loops through the list and finds what are KillXEnemiesQuests and updates them. Needs to check what enemy is killed with placeholder enemy var
  (cast `/Game/FirstPerson/Blueprints/BP_FirstPersonCharacter` (`self.GetOwner`))
  (for _array_element (`self.Quests`)
    (bind _asbp_kill_xenemies_quest (cast `/Game/Blueprints/NPC/Quests/BP_KillXEnemiesQuest` _array_element))
    (`/Engine/EditorBlueprintResources/StandardMacros.IncrementInt` (`/Game/Blueprints/NPC/Quests/BP_KillXEnemiesQuest.EnemiesKilled` _asbp_kill_xenemies_quest)
      (:`  `
        (`/Game/Blueprints/NPC/Quests/BP_Quest.CheckQuestCompletion` _asbp_kill_xenemies_quest)
        (break)))))

(event `Key|P`
  (params (Key :type "Key Structure"))
  ;[1 1 1] Test to see if the NPC is changing states properly
  (:`Pressed`
    (cast `/Game/FirstPerson/Blueprints/BP_FirstPersonCharacter` (`self.GetOwner`))
    (for _array_element (`self.Quests`)
      (if (`/Game/Blueprints/NPC/Quests/BP_Quest.IsQuestActive` _array_element)
        (set `/Game/Blueprints/NPC/Quests/BP_Quest.IsQuestComplete` true _array_element)))))