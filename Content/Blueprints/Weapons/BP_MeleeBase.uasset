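; Base melee weapon Blueprint that plays a first-person attack animation when the item is used.
; OnUseItem is gated by a CanAttack flag, which re-enables after a delay equal to the inverse of the Attack Speed property.
; Attack plays AttackMontage on the character's first-person mesh at the rate of the Speed property.
; Both values are looked up by name with fallback defaults, and no hit detection or damage is handled here.
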(event `self.OnUseItem`
  ;[1 1 1] Use Weapon
  (if (`self.CanAttack`)
    (`self.Attack`)
    (set `self.CanAttack` false)
    (`KismetSystemLibrary.Delay` (/ 1.0 (`self.GetProperty` "Attack Speed" 1.5)))
    (set `self.CanAttack` true)))

(fn `Attack`
  (`AnimInstance.Montage_Play` (`self.GetAnimInstance` (`/Game/FirstPerson/Blueprints/BP_FirstPersonCharacter.FirstPersonMesh` (`self.First PersonCharacter`))) (`self.AttackMontage`) (`self.GetProperty` "Speed" 1.0) "MontageLength" 0.0 true))