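; BP_SwordBase is a sword weapon item that performs a melee swing when used, with no hit or damage logic in this file.
; OnUseItem calls Attack, which plays a sword attack montage on the first-person character's mesh, then locks further attacks behind a CanAttack flag.
; A Delay driven by the item's "Attack Speed" property clears that lock, so the value acts as a cooldown in seconds.
; OnReleaseItem is empty, and debug prints remain.
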(event `self.OnUseItem`
  (if (`self.CanAttack`)
    (`KismetSystemLibrary.PrintString` "Hello")
    (`self.Attack`)
    (set `self.CanAttack` false)
    (`KismetSystemLibrary.Delay` (/ (`self.GetProperty` "Attack Speed" 1.5) 1.0))
    (set `self.CanAttack` true)))

(event `self.OnReleaseItem`)

(fn `Attack`
  (`KismetSystemLibrary.PrintString` "Good")
  (`AnimInstance.Montage_Play` (`self.GetAnimInstance` (`/Game/FirstPerson/Blueprints/BP_FirstPersonCharacter.FirstPersonMesh` (`self.First PersonCharacter`))) "/Game/Animations/Sword_Animation/SK_Sword_Attack1_V6_Mont.SK_Sword_Attack1_V6_Mont" 1.0 "MontageLength" 0.0 true))