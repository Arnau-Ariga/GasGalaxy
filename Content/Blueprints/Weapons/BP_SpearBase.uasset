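; Base spear weapon Blueprint that plays a first-person attack animation when the item is used.
; OnUseItem calls Attack, which plays the spear attack montage on the character's first-person mesh.
; A CanAttack flag and a Delay driven by the "Attack Speed" property act as the cooldown between attacks.
; Releasing the item does nothing, and this file contains no hit or damage logic.
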(event `self.OnUseItem`
  (if (`self.CanAttack`)
    (`self.Attack`)
    (set `self.CanAttack` false)
    (`KismetSystemLibrary.Delay` (/ (`self.GetProperty` "Attack Speed" 1.5) 1.0))
    (set `self.CanAttack` true)))

(event `self.OnReleaseItem`)

(fn `Attack`
  (`AnimInstance.Montage_Play` (`self.GetAnimInstance` (`/Game/FirstPerson/Blueprints/BP_FirstPersonCharacter.FirstPersonMesh` (`self.First PersonCharacter`))) "/Game/Animations/Spear_Animation/SK_Spear_Attack_Montage.SK_Spear_Attack_Montage" 1.0 "MontageLength" 0.0 true))