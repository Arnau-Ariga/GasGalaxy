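; Base weapon projectile whose speed, gravity, bounciness, size and elemental Niagara trail are set in the construction script from its properties.
; On hit, it applies a knockback impulse and damage only to physics-simulating components, then destroys itself unless SurviveHit is set.
; Destruction by any cause calls Explode, which spawns BP_Explosion with the projectile's damage when ExplosionRadius is above zero.
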(event `self.ReceiveHit`
  (params (MyComp :type "PrimitiveComponent Object Reference") (Other :type "Actor Object Reference") (OtherComp :type "PrimitiveComponent Object Reference") (bSelfMoved :type Boolean) (HitLocation :type "Vector Structure") (HitNormal :type "Vector Structure") (NormalImpulse :type "Vector Structure") (Hit :type "HitResult Structure (by ref)"))
  ;[1 1 1] Projectile Hit
  (if (`SceneComponent.IsSimulatingPhysics` OtherComp "None")
    (`PrimitiveComponent.AddImpulseAtLocation` OtherComp (* (`self.GetVelocity`) (`self.Knockback`) 100.0) (`self.K2_GetActorLocation`) "None")
    (`GameplayStatics.ApplyDamage` Other (`self.Damage`) null self))
  (if (not (`self.SurviveHit`))
    (`self.K2_DestroyActor`)))

(event `Explode`
  ;[1 1 1] Explode If Applicable
  (if (> (`self.ExplosionRadius`) 0.0)
    (`|SpawnActorFromClass` "/Game/Blueprints/Weapons/Projectiles/BP_Explosion.BP_Explosion_C" (`KismetMathLibrary.Conv_VectorToTransform` (`self.K2_GetActorLocation`)) "Undefined" "MultiplyWithRoot" null (`self.Damage`) (`self.ExplosionRadius`) null)))

(event `self.ReceiveDestroyed`
  (`self.Explode`))

(fn `UserConstructionScript`
  (bind _projectilemovement (`self.ProjectileMovement`))
  (`|ExecutionSequence`
    (:`then_0`
      ;[1 1 1] Set Particle Trail
      (`NiagaraComponent.SetAsset` (`self.ProjectileTrail`) (`|GetArrayItem` (`|MakeArray` "/Game/Blueprints/Weapons/Projectiles/Effects/NS_BasicProjectileTrail.NS_BasicProjectileTrail" "/Game/Blueprints/Weapons/Projectiles/Effects/NS_FireProjectileTrail.NS_FireProjectileTrail" "/Game/Blueprints/Weapons/Projectiles/Effects/NS_OilProjectileTrail.NS_OilProjectileTrail" "/Game/Blueprints/Weapons/Projectiles/Effects/NS_IceProjectileTrail.NS_IceProjectileTrail" "/Game/Blueprints/Weapons/Projectiles/Effects/NS_RockProjectileTrail.NS_RockProjectileTrail" "/Game/Blueprints/Weapons/Projectiles/Effects/NS_WindProjectileTrail.NS_WindProjectileTrail" :!type "NiagaraSystem Object Reference") (`KismetMathLibrary.Conv_ByteToInt` (`self.ElementalType`))) true))
    (:`then_1`
      ;[1 1 1] Set Properties
      (set `ProjectileMovementComponent.InitialSpeed` (* (`self.Speed`) 1000.0) _projectilemovement)
      (set `ProjectileMovementComponent.ProjectileGravityScale` (`self.GravityScale`) _projectilemovement)
      (set `ProjectileMovementComponent.Bounciness` (`self.Bounciness`) _projectilemovement)
      (`SceneComponent.SetRelativeScale3D` (`self.CollisionComponent`) (`KismetMathLibrary.Conv_DoubleToVector` (`self.Size`))))))