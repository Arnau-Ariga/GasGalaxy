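; Explosion actor that plays an explosion sound at its location on BeginPlay and applies damage through an overlap trigger.
; The construction script sizes the Trigger sphere from the Radius variable scaled up tenfold.
; Begin-overlap events on that sphere call ApplyDamage with the Damage value and itself as causer, and the actor destroys itself when the Explosion particle system finishes.
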(event `self.ReceiveBeginPlay`
  (`GameplayStatics.PlaySoundAtLocation` "/Game/StarterContent/Audio/Explosion_Cue.Explosion_Cue" (`self.K2_GetActorLocation`) (struct) 1.0 1.0 0.0 null null null null))

(event `self.Trigger.OnComponentBeginOverlap`
  (params (OverlappedComponent :type "PrimitiveComponent Object Reference") (OtherActor :type "Actor Object Reference") (OtherComp :type "PrimitiveComponent Object Reference") (OtherBodyIndex :type Integer) (bFromSweep :type Boolean) (SweepResult :type "HitResult Structure (by ref)"))
  (`GameplayStatics.ApplyDamage` null (`self.Damage`) null self))

(event `self.Explosion.OnSystemFinished`
  (params (PSystem :type "NiagaraComponent Object Reference"))
  (`self.K2_DestroyActor`))

(fn `UserConstructionScript`
  (`SphereComponent.SetSphereRadius` (`self.Trigger`) (* (`self.Radius`) 10.0) true))