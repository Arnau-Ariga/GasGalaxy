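; Melee hit component that detects pawns struck by the first-person weapon and damages them.
; HitDetect reads HoldingPose from the first-person AnimBP to choose a sword box trace or spear sphere trace.
; Each is a zero-length trace at the weapon's mesh socket, testing only the current position rather than sweeping the swing.
; A valid hit receives ApplyDamage using the equipped item's Damage property; spear trace radius also comes from item properties.
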(event `HitDetect`
  (params (FirstPersonMesh :type "SkeletalMeshComponent Object Reference"))
  ;[1 1 1] Hit Detection
  (bind _asfirst_person_anim_bp (cast `/Game/FirstPersonArms/Animations/FirstPerson_AnimBP` (`SkeletalMeshComponent.GetAnimInstance` FirstPersonMesh)))
  (bind _hitactor (`self.DetectHit` (`/Game/FirstPersonArms/Animations/FirstPerson_AnimBP.HoldingPose` _asfirst_person_anim_bp) FirstPersonMesh))
  (`/Engine/EditorBlueprintResources/StandardMacros.IsValid` _hitactor
    (:`Is Valid`
      (`self.DamageActor` _hitactor))))

(event `DamageActor`
  (params (Actor :type "Actor Object Reference"))
  ;[1 1 1] Damage Hit Actor
  (`GameplayStatics.ApplyDamage` Actor (`/Game/Blueprints/Equipment/BP_EquipmentBase.GetProperty` (`/Game/Blueprints/Inventory/BP_Inventory.EquippedItem` (`/Game/Blueprints/Inventory/FL_InventoryFunctions.GetInventory`)) "Damage" 1.0) null null "/Script/Engine.DamageType"))

(fn `DetectHit`
  (params (HoldingPose :type "/Game/Blueprints/Equipment/E_EquipmentPose Enum" :default "NewEnumerator3") (FirstPersonMesh :type "SkeletalMeshComponent Object Reference"))
  (returns (HitActor :type "Actor Object Reference"))
  (switch `/Game/Blueprints/Equipment/E_EquipmentPose` HoldingPose
    (:`NewEnumerator1`
      (bind _hitactor (`self.SwordHitDetect` FirstPersonMesh))
      (return _hitactor))
    (:`NewEnumerator2`
      (bind _hitactor_2 (`self.SpearHitDetect` FirstPersonMesh))
      (return _hitactor_2))))

(fn `SpearHitDetect`
  (params (FirstPersonMesh :type "SkeletalMeshComponent Object Reference"))
  (returns (HitActor :type "Actor Object Reference"))
  (bind _returnvalue (`SceneComponent.GetSocketLocation` FirstPersonMesh "spear_socket"))
  (bind _outhit (`KismetSystemLibrary.SphereTraceSingleForObjects` :`Start` _returnvalue :`End` _returnvalue :`Radius` (`/Game/Blueprints/Equipment/BP_EquipmentBase.GetProperty` (`/Game/Blueprints/Inventory/BP_Inventory.EquippedItem` (`/Game/Blueprints/Inventory/FL_InventoryFunctions.GetInventory`)) "Radius" 10.0) :`ObjectTypes` (`|MakeArray` "ObjectTypeQuery3" :!type "EObjectTypeQuery Enum") :`DrawTime` 0.5))
  (return (`.HitActor` (`GameplayStatics.BreakHitResult` _outhit))))

(fn `SwordHitDetect`
  (params (FirstPersonMesh :type "SkeletalMeshComponent Object Reference"))
  (returns (HitActor :type "Actor Object Reference"))
  (bind _returnvalue (`SceneComponent.GetSocketLocation` FirstPersonMesh "blade_socket"))
  (bind _outhit (`KismetSystemLibrary.BoxTraceSingleForObjects` :`Start` _returnvalue :`End` _returnvalue :`HalfSize` (1.0 1.0 75.0) :`Orientation` (`SceneComponent.GetSocketRotation` FirstPersonMesh "blade_socket") :`ObjectTypes` (`|MakeArray` "ObjectTypeQuery3" :!type "EObjectTypeQuery Enum") :`DrawTime` 0.5))
  (return (`.HitActor` (`GameplayStatics.BreakHitResult` _outhit))))