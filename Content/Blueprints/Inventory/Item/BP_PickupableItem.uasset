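; A pickupable item in the world that the player can add to the inventory.
; Its construction script sets the mesh from the item name, sizes the module array to that item's slot count and constructs a BP_ItemInstance from both.
; GetPrompt builds a "Pick Up" prompt with the item's name, and PickUp passes the instance to the inventory and returns the result.
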(fn `GetPrompt`
  (returns (Prompt :type String))
  (return (`KismetStringLibrary.Concat_StrStr` "Pick Up " (`KismetStringLibrary.Conv_NameToString` (`/Game/Blueprints/Inventory/Item/BP_ItemInstance.ItemName` (`self.Item`))))))

(fn `PickUp`
  (returns (PickedUp :type Boolean))
  (bind _itemadded (`/Game/Blueprints/Inventory/FL_InventoryFunctions.AddItemToInventory` (`self.Item`)))
  (return _itemadded))

(fn `UserConstructionScript`
  (bind _itemname (`self.ItemName`))
  (`StaticMeshComponent.SetStaticMesh` (`self.Mesh`) (`/Game/Blueprints/Inventory/Item/FL_ItemFunctions.GetItemMesh` (`self.ItemName`)))
  ;[1 1 1] Create Item Instance
  (`KismetArrayLibrary.Array_Resize` (`self.Modules`) (`/Game/Blueprints/Inventory/Item/FL_ItemFunctions.GetItemModuleSlots` _itemname))
  (bind _returnvalue (`|GenericCreateObject` "/Game/Blueprints/Inventory/Item/BP_ItemInstance.BP_ItemInstance_C" _itemname (`self.Modules`)))
  (set `self.Item` _returnvalue))