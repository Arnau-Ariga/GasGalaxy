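; Blueprint function library that gives global access to the player's inventory.
; GetInventory casts player pawn 0 to BP_FirstPersonCharacter and returns its Inventory, and every other function forwards to that object.
; Wrappers cover slot items (get, add, remove, swap, search), counted key items, item modules and the currently equipped item with a validity flag.
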(fn `AddItemToInventory`
  (params (Item :type "/Game/Blueprints/Inventory/Item/BP_ItemInstance Object Reference"))
  (returns (ItemAdded :type Boolean))
  (bind _itemadded (`/Game/Blueprints/Inventory/BP_Inventory.AddItem` (`self.GetInventory` (`local.__WorldContext`)) Item))
  (return _itemadded))

(fn `AddKeyItemToInventory`
  (params (KeyItemName :type Name) (Count :type Integer :default 1))
  (`/Game/Blueprints/Inventory/BP_Inventory.AddKeyItem` (`self.GetInventory` (`local.__WorldContext`)) KeyItemName Count)
  (return))

(fn `AddModuleToInventory`
  (params (ModuleName :type Name))
  (returns (ModuleAdded :type Boolean))
  (bind _moduleadded (`/Game/Blueprints/Inventory/BP_Inventory.AddModule` (`self.GetInventory` (`local.__WorldContext`)) ModuleName))
  (return _moduleadded))

(fn `GetEquippedItemFromInventory`
  (returns (Item :type "/Game/Blueprints/Inventory/Item/BP_ItemInstance Object Reference") (IsValid :type Boolean))
  (bind _inventory (`self.GetInventory` (`local.__WorldContext`)))
  (bind _item (`/Game/Blueprints/Inventory/BP_Inventory.GetItem` _inventory (`/Game/Blueprints/Inventory/BP_Inventory.EquippedItemSlotIndex` _inventory)))
  (return _item (`KismetSystemLibrary.IsValid` _item)))

(fn `GetInventory`
  (returns (Inventory :type "/Game/Blueprints/Inventory/BP_Inventory Object Reference"))
  (bind _asbp_first_person_character (cast `/Game/FirstPerson/Blueprints/BP_FirstPersonCharacter` (`GameplayStatics.GetPlayerPawn` null)))
  (return (`/Game/FirstPerson/Blueprints/BP_FirstPersonCharacter.Inventory` _asbp_first_person_character)))

(fn `GetItemFromInventory`
  (params (ItemSlotIndex :type Integer))
  (returns (Item :type "/Game/Blueprints/Inventory/Item/BP_ItemInstance Object Reference"))
  (return (`/Game/Blueprints/Inventory/BP_Inventory.GetItem` (`self.GetInventory` (`local.__WorldContext`)) ItemSlotIndex)))

(fn `GetKeyItemCountFromInventory`
  (params (KeyItemName :type Name))
  (returns (Count :type Integer))
  (return (`/Game/Blueprints/Inventory/BP_Inventory.GetKeyItemCount` (`self.GetInventory` (`local.__WorldContext`)) KeyItemName)))

(fn `InventoryContainsItem`
  (params (ItemName :type Name))
  (returns (ItemSlotIndex :type Integer) (Contains :type Boolean))
  (bind (_itemslotindex _contains) (`/Game/Blueprints/Inventory/BP_Inventory.ContainsItem` (`self.GetInventory` (`local.__WorldContext`)) ItemName))
  (return _itemslotindex _contains))

(fn `RemoveItemFromInventory`
  (params (ItemSlotIndex :type Integer))
  (returns (Item :type "/Game/Blueprints/Inventory/Item/BP_ItemInstance Object Reference"))
  (locals (ItemNameToReturn :type Name))
  (bind _item (`/Game/Blueprints/Inventory/BP_Inventory.RemoveItem` (`self.GetInventory` (`local.__WorldContext`)) ItemSlotIndex))
  (return _item))

(fn `RemoveKeyItemFromInventory`
  (params (KeyItemName :type Name) (Count :type Integer :default 1))
  (returns (WasRemoved :type Boolean))
  (bind _wasremoved (`/Game/Blueprints/Inventory/BP_Inventory.RemoveKeyItem` (`self.GetInventory` (`local.__WorldContext`)) KeyItemName Count))
  (return _wasremoved))

(fn `RemoveModuleFromInventory`
  (params (ItemSlotIndex :type Integer) (ModuleSlotIndex :type Integer))
  (returns (ModuleName :type Name))
  (locals (ItemNameToReturn :type Name))
  (bind _modulename (`/Game/Blueprints/Inventory/BP_Inventory.RemoveModule` (`self.GetInventory` (`local.__WorldContext`)) ItemSlotIndex ModuleSlotIndex))
  (return _modulename))

(fn `SwapItemsInInventory`
  (params (ItemSlotIndex1 :type Integer) (ItemSlotIndex2 :type Integer))
  (returns (SwapSuccessful :type Boolean))
  (bind _swapsuccessful (`/Game/Blueprints/Inventory/BP_Inventory.SwapItems` (`self.GetInventory` (`local.__WorldContext`)) ItemSlotIndex1 ItemSlotIndex2))
  (return _swapsuccessful))