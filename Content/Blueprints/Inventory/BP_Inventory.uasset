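; Player inventory component that stores typed item slots, per-item modules and counted key items, and grants a starter loadout on BeginPlay.
; It creates the inventory widget and adds an input mapping, with the open action showing the UI and pausing the game.
; Hotkeys equip fixed slots by unequipping the current item and adding that item's equipment component class to the owner.
; Items only enter or swap between type-matched slots, with swaps updating the equipped index.
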(event `self.ReceiveBeginPlay`
  (bind _returnvalue (pcsubsystem `EnhancedInputLocalPlayerSubsystem` (`GameplayStatics.GetPlayerController` 0)))
  (`|ExecutionSequence`
    (:`then_0`
      ;[1 1 1] Create Inventroy Widget
      (bind _returnvalue_2 (`|CreateWidget` "/Game/Blueprints/Inventory/UI/W_Inventory.W_Inventory_C" (`GameplayStatics.GetPlayerController` 0)))
      (set `self.Inventory` _returnvalue_2))
    (:`then_1`
      ;[1 1 1] Add Invetory Mapping Context To Player Controller
      (`/Engine/EditorBlueprintResources/StandardMacros.IsValid` _returnvalue
        (:`Is Valid`
          (`EnhancedInputSubsystemInterface.AddMappingContext` _returnvalue "/Game/Blueprints/Inventory/Input/IMC_Inventory.IMC_Inventory" 1 (struct)))))
    (:`then_2`
      (`self.GiveStarterLoadout`))))

(event `EnhancedInput|/Game/Blueprints/Inventory/Input/IA_OpenInventory`
  (params (ActionValue :type Boolean) (ElapsedSeconds :type "Float (double-precision)") (TriggeredSeconds :type "Float (double-precision)") (InputAction :type "InputAction Object Reference" :default "/Game/Blueprints/Inventory/Input/IA_OpenInventory.IA_OpenInventory"))
  (bind _returnvalue (`GameplayStatics.GetPlayerController` 0))
  (bind _inventory (`self.Inventory`))
  ;[1 1 1] Open Inventory
  (:`Triggered`
    (`UserWidget.AddToViewport` _inventory 0)
    (`WidgetBlueprintLibrary.SetInputMode_UIOnlyEx` _returnvalue _inventory)
    (set `PlayerController.bShowMouseCursor` true _returnvalue)
    (`GameplayStatics.SetGamePaused` true)))

(event `EquipItem`
  (params (`Item Slot Index` :type Integer))
  (bind _item (`self.GetItem` `Item Slot Index`))
  (bind _equipmentcomponent (`/Game/Blueprints/Inventory/Item/FL_ItemFunctions.GetItemEquipmentComponent` (`/Game/Blueprints/Inventory/Item/BP_ItemInstance.ItemName` _item)))
  ;[1 1 1] Equip Item
  (`self.UnequipEquippedItem`)
  (`/Engine/EditorBlueprintResources/StandardMacros.IsValid` _item
    (:`Is Valid`
      (if (`KismetSystemLibrary.IsValidClass` _equipmentcomponent)
        (bind _returnvalue (`|AddComponentByClass` :`self` (`self.GetOwner`) :`Class` _equipmentcomponent))
        (set `self.EquippedItem` _returnvalue)
        (set `self.EquippedItemSlotIndex` `Item Slot Index`)))))

(event `UnequipEquippedItem`
  (bind _equippeditem (`self.EquippedItem`))
  ;[1 1 1] Unequip Equipped Item
  (`/Engine/EditorBlueprintResources/StandardMacros.IsValid` _equippeditem
    (:`Is Valid`
      (`/Game/Blueprints/Equipment/BP_EquipmentBase.Unequip` _equippeditem))))

(event `EnhancedInput|/Game/Blueprints/Inventory/Input/IA_EquipGun1`
  (params (ActionValue :type Boolean) (ElapsedSeconds :type "Float (double-precision)") (TriggeredSeconds :type "Float (double-precision)") (InputAction :type "InputAction Object Reference" :default "/Game/Blueprints/Inventory/Input/IA_EquipGun1.IA_EquipGun1"))
  ;[1 1 1] Equip Items
  (:`Triggered`
    (`self.EquipItem` 2)))

(event `EnhancedInput|/Game/Blueprints/Inventory/Input/IA_EquipGun2`
  (params (ActionValue :type Boolean) (ElapsedSeconds :type "Float (double-precision)") (TriggeredSeconds :type "Float (double-precision)") (InputAction :type "InputAction Object Reference" :default "/Game/Blueprints/Inventory/Input/IA_EquipGun2.IA_EquipGun2"))
  ;[1 1 1] Equip Items
  (:`Triggered`
    (`self.EquipItem` 3)))

(event `EnhancedInput|/Game/Blueprints/Inventory/Input/IA_EquipMelee`
  (params (ActionValue :type Boolean) (ElapsedSeconds :type "Float (double-precision)") (TriggeredSeconds :type "Float (double-precision)") (InputAction :type "InputAction Object Reference" :default "/Game/Blueprints/Inventory/Input/IA_EquipMelee.IA_EquipMelee"))
  ;[1 1 1] Equip Items
  (:`Triggered`
    (`self.EquipItem` 4)))

(event `GiveStarterLoadout`
  ;[1 1 1] Give Starter Loadout
  (bind _returnvalue (`|GenericCreateObject` "/Game/Blueprints/Inventory/Item/BP_ItemInstance.BP_ItemInstance_C" "Assault Rifle" (`|MakeArray` "Cherries" "None" "None" "None" :!type "Name")))
  (`self.AddItem` _returnvalue)
  (bind _returnvalue_2 (`|GenericCreateObject` "/Game/Blueprints/Inventory/Item/BP_ItemInstance.BP_ItemInstance_C" "Shotgun" (`|MakeArray` "Quick Fire" "None" "None" :!type "Name")))
  (`self.AddItem` _returnvalue_2)
  (bind _returnvalue_3 (`|GenericCreateObject` "/Game/Blueprints/Inventory/Item/BP_ItemInstance.BP_ItemInstance_C" "Metal Sword" (`|MakeArray` "Feathers" "None" :!type "Name")))
  (`self.AddItem` _returnvalue_3))

(fn `AddItem`
  (params (Item :type "/Game/Blueprints/Inventory/Item/BP_ItemInstance Object Reference"))
  (returns (ItemAdded :type Boolean))
  (locals (SlotIndex :type Integer :default -1))
  ;[1 1 1] Find Empty Slot Of Type
  (for (_array_element _array_index) (`self.ItemSlots`)
    (bind (_item _type) (break `/Game/Blueprints/Inventory/S_ItemSlot` _array_element))
    (`/Engine/EditorBlueprintResources/StandardMacros.IsValid` _item
      (:`Is Not Valid`
        (if (`|EnumEquality` _type (`/Game/Blueprints/Inventory/Item/FL_ItemFunctions.GetItemType` (`/Game/Blueprints/Inventory/Item/BP_ItemInstance.ItemName` Item)))
          (set `local.SlotIndex` _array_index)
          (break)))))
  ;[1 1 1] Add Item To Slot If Found
  (if (>= (`local.SlotIndex`) 0)
    (setmembers `/Game/Blueprints/Inventory/S_ItemSlot` :`StructRef` (`|GetArrayItem` (`self.ItemSlots`) (`local.SlotIndex`)) :`Item` Item)
    (return true)))

(fn `AddKeyItem`
  (params (KeyItemName :type Name) (Count :type Integer :default 1))
  (`BlueprintMapLibrary.Map_Add` (`self.KeyItems`) KeyItemName (+ (`BlueprintMapLibrary.Map_Find` (`self.KeyItems`) KeyItemName) Count))
  (`/Game/Blueprints/Inventory/UI/W_KeyItemsMenu.AddKeyItem` (`/Game/Blueprints/Inventory/UI/W_Inventory.W_KeyItemsMenu` (`self.Inventory`)) KeyItemName))

(fn `AddModule`
  (params (ModuleName :type Name))
  (returns (ModuleAdded :type Boolean))
  (locals (SlotIndex :type Integer :default -1))
  (for _array_element (`self.ItemSlots`)
    (bind _moduleadded (`/Game/Blueprints/Equipment/Module/FL_ModuleFunctions.AddModuleToItem` (`.Item_17_6AA6CCEB454C3815FF6FE3928A75E6E0` (break `/Game/Blueprints/Inventory/S_ItemSlot` _array_element)) ModuleName))
    (if _moduleadded
      (return true))))

(fn `ContainsItem`
  (params (ItemName :type Name :default "None"))
  (returns (ItemSlotIndex :type Integer) (Contains :type Boolean))
  (locals (FoundSlotIndex :type Integer :default -1))
  (for (_array_element _array_index) (`self.ItemSlots`)
    (if (== (`/Game/Blueprints/Inventory/Item/BP_ItemInstance.ItemName` (`.Item_17_6AA6CCEB454C3815FF6FE3928A75E6E0` (break `/Game/Blueprints/Inventory/S_ItemSlot` _array_element))) ItemName)
      (set `local.FoundSlotIndex` _array_index)
      (return (`local.FoundSlotIndex`) true))))

(fn `GetItem`
  (params (ItemSlotIndex :type Integer))
  (returns (Item :type "/Game/Blueprints/Inventory/Item/BP_ItemInstance Object Reference"))
  (return (`.Item_17_6AA6CCEB454C3815FF6FE3928A75E6E0` (break `/Game/Blueprints/Inventory/S_ItemSlot` (`|GetArrayItem` (`self.ItemSlots`) ItemSlotIndex)))))

(fn `GetKeyItemCount`
  (params (KeyItemName :type Name))
  (returns (Count :type Integer))
  (return (`BlueprintMapLibrary.Map_Find` (`self.KeyItems`) KeyItemName)))

(fn `RemoveItem`
  (params (SlotIndex :type Integer))
  (returns (Item :type "/Game/Blueprints/Inventory/Item/BP_ItemInstance Object Reference"))
  (locals (ItemToReturn :type "/Game/Blueprints/Inventory/Item/BP_ItemInstance Object Reference"))
  (if (== (`self.EquippedItemSlotIndex`) SlotIndex)
    (`self.UnequipEquippedItem`))
  (bind _output_get (set `local.ItemToReturn` (`.Item_17_6AA6CCEB454C3815FF6FE3928A75E6E0` (break `/Game/Blueprints/Inventory/S_ItemSlot` (`|GetArrayItem` (`self.ItemSlots`) SlotIndex)))))
  (setmembers `/Game/Blueprints/Inventory/S_ItemSlot` :`StructRef` (`|GetArrayItem` (`self.ItemSlots`) SlotIndex) :`Item` null)
  (return _output_get))

(fn `RemoveKeyItem`
  (params (KeyItemName :type Name) (Count :type Integer :default 1))
  (returns (WasRemoved :type Boolean))
  (bind _value (`BlueprintMapLibrary.Map_Find` (`self.KeyItems`) KeyItemName))
  (if (>= _value Count)
    (`BlueprintMapLibrary.Map_Add` (`self.KeyItems`) KeyItemName (- _value Count))
    (return true)))

(fn `RemoveModule`
  (params (ItemSlotIndex :type Integer) (ModuleSlotIndex :type Integer))
  (returns (ModuleName :type Name))
  (locals (ModuleNameToReturn :type Name))
  (bind _modules (`/Game/Blueprints/Inventory/Item/BP_ItemInstance.Modules` (`.Item_17_6AA6CCEB454C3815FF6FE3928A75E6E0` (break `/Game/Blueprints/Inventory/S_ItemSlot` (`|GetArrayItem` (`self.ItemSlots`) ItemSlotIndex)))))
  (bind _output_get (set `local.ModuleNameToReturn` (`|GetArrayItem` _modules ModuleSlotIndex)))
  (`KismetArrayLibrary.Array_Set` _modules ModuleSlotIndex)
  (return _output_get))

(fn `SwapItems`
  (params (ItemSlotIndex1 :type Integer) (ItemSlotIndex2 :type Integer))
  (returns (SwapSuccessful :type Boolean))
  (bind _itemslots (`self.ItemSlots`))
  (if (`|EnumEquality` (`.Type_5_0C0084804C6F6A0400A55F9B354A9F0B` (break `/Game/Blueprints/Inventory/S_ItemSlot` (`|GetArrayItem` _itemslots ItemSlotIndex1))) (`.Type_5_0C0084804C6F6A0400A55F9B354A9F0B` (break `/Game/Blueprints/Inventory/S_ItemSlot` (`|GetArrayItem` _itemslots ItemSlotIndex2))))
    (`KismetArrayLibrary.Array_Swap` (`self.ItemSlots`) ItemSlotIndex1 ItemSlotIndex2)
    ;[1 1 1] Swap Equipped Item Slot Index If Applicable
    (if (== (`self.EquippedItemSlotIndex`) ItemSlotIndex1)
      (set `self.EquippedItemSlotIndex` ItemSlotIndex2)
      (elif (== (`self.EquippedItemSlotIndex`) ItemSlotIndex2)
        (set `self.EquippedItemSlotIndex` ItemSlotIndex1)))
    (return true)))