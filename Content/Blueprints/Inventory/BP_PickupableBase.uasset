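; Base pickupable item actor for the inventory, with a mesh that spins slowly around its yaw axis every Tick.
; On Interact it calls PickUp, then either plays a sound and destroys itself on success or sends a "Not Enough Room" pop-up on failure.
; PickUp, GetPrompt and IsInteractable hold only placeholder defaults here: always succeeds, empty prompt and always interactable.
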(event `self.ReceiveTick`
  (params (DeltaSeconds :type "Float (single-precision)"))
  ;[1 1 1] Rotate Mesh
  (`SceneComponent.K2_AddWorldRotation` (`self.Mesh`) (`KismetMathLibrary.MakeRotator` 0.0 0.0 (* DeltaSeconds 50.0)) false false))

(event `/Game/Blueprints/Interact/BPI_Interactable.Interact`
  ;[1 1 1] Pick Up
  (bind _pickedup (`self.PickUp`))
  (if _pickedup
    (`GameplayStatics.PlaySoundAtLocation` "/Game/SoundEffects/Cues/Pickup_Cue.Pickup_Cue" (`SceneComponent.K2_GetComponentLocation` (`self.DefaultSceneRoot`)) (struct) 1.0 1.0 0.0 null null null null)
    (`self.K2_DestroyActor`)
    (else
      (`/Game/Blueprints/PopUp/FL_PopUpFunctions.SendPopUp` "/Game/Textures/Images/Icons/WhiteBackpackIcon.WhiteBackpackIcon" "Not Enough Room"))))

(fn `GetPrompt`
  (returns (Prompt :type String))
  (return ""))

(fn `IsInteractable`
  (returns (IsInteractable :type Boolean))
  (return true))

(fn `PickUp`
  (returns (PickedUp :type Boolean))
  (return true))

(fn `UserConstructionScript`)