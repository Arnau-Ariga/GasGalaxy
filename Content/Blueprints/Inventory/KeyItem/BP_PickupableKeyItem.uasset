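; BP_PickupableKeyItem is a pickup actor that adds a key item to the inventory.
; Its construction script uses KeyItemName to look up and apply the item's mesh and particle color, so one Blueprint represents any key item.
; GetPrompt builds a "Pick Up" label from the item name, and PickUp adds one of that item and returns true.
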(fn `GetPrompt`
  (returns (Prompt :type String))
  (return (`KismetStringLibrary.Concat_StrStr` "Pick Up " (`KismetStringLibrary.Conv_NameToString` (`self.KeyItemName`)))))

(fn `PickUp`
  (returns (PickedUp :type Boolean))
  (`/Game/Blueprints/Inventory/FL_InventoryFunctions.AddKeyItemToInventory` (`self.KeyItemName`))
  (return true))

(fn `UserConstructionScript`
  (bind _keyitemname (`self.KeyItemName`))
  (`StaticMeshComponent.SetStaticMesh` (`self.Mesh`) (`/Game/Blueprints/Inventory/KeyItem/FL_KeyItemFunctions.GetKeyItemMesh` _keyitemname))
  (`NiagaraComponent.SetVariableLinearColor` (`self.Particles`) "Color" (`/Game/Blueprints/Inventory/KeyItem/FL_KeyItemFunctions.GetKeyItemParticleColor` _keyitemname)))