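; Component that manages the player's inventory of throwables, such as grenades, and handles readying and throwing them.
; Pickups append their class to an array that works as a first-in, first-out queue.
; Readying spawns the first queued class at the component's transform on the player.
; Throwing launches that actor along the player controller's forward vector at its own throw speed by activating its movement component, then removes the queue entry.
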(event `ReadyThrowable`
  (if (> (`KismetArrayLibrary.Array_Length` (`self.ThrowableTypes`)) 0)
    (bind _returnvalue (`|SpawnActorFromClass` (`|GetArrayItem` (`self.ThrowableTypes`)) (`self.K2_GetComponentToWorld` (`/Game/FirstPerson/Blueprints/BP_FirstPersonCharacter.BPC_Throwable` (`self.Player`))) "Undefined" "MultiplyWithRoot" null null))
    (set `self.CurrentThrowable` _returnvalue)))

(event `ThrowThrowable`
  (bind _currentthrowable (`self.CurrentThrowable`))
  (bind _throwablemovement (`/Game/Blueprints/Throwables/BP_Throwable_Base.ThrowableMovement` _currentthrowable))
  (if (> (`KismetArrayLibrary.Array_Length` (`self.ThrowableTypes`)) 0)
    (set `MovementComponent.Velocity` (* (`Actor.GetActorForwardVector` (`GameplayStatics.GetPlayerController` 0)) (`/Game/Blueprints/Throwables/BP_Throwable_Base.ThrowSpeed` _currentthrowable)) _throwablemovement)
    (`self.Activate` _throwablemovement false)
    (`KismetArrayLibrary.Array_Remove` (`self.ThrowableTypes`))))

(event `nadePickedUp`
  (params (nadeType :type "/Game/Blueprints/Throwables/BP_Throwable_Base Class Reference"))
  (`KismetArrayLibrary.Array_Add` (`self.ThrowableTypes`) nadeType))