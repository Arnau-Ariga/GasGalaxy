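; BP_Oil_Nade is a throwable oil grenade that leaves a BP_OilPuddle where it goes off.
; It calls Detonate only when a projectile bounce hits a nearly flat, upward-facing surface.
; The Effect override spawns the puddle at the collider's transform, then calls the parent Effect.
; Overlapping an actor tagged OilPuddle clears HasEffect.
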(event `self.ThrowableCollider.OnComponentBeginOverlap`
  (params (OverlappedComponent :type "PrimitiveComponent Object Reference") (OtherActor :type "Actor Object Reference") (OtherComp :type "PrimitiveComponent Object Reference") (OtherBodyIndex :type Integer) (bFromSweep :type Boolean) (SweepResult :type "HitResult Structure (by ref)"))
  (if (`self.ActorHasTag` OtherActor "OilPuddle")
    (set `self.hasEffect` false)))

(event `self.ThrowableMovement.OnProjectileBounce`
  (params (ImpactResult :type "HitResult Structure (by ref)") (ImpactVelocity :type "Vector Structure (by ref)"))
  (if (== (`.ImpactNormal` (`GameplayStatics.BreakHitResult` ImpactResult)) (0.0 0.0 1.0) :`ErrorTolerance` 0.2)
    (`self.Detonate`)))

(fn `Effect`
  (`|SpawnActorFromClass` "/Game/Blueprints/Oil/BP_OilPuddle.BP_OilPuddle_C" (`SceneComponent.K2_GetComponentToWorld` (`self.ThrowableCollider`)) "Undefined" "MultiplyWithRoot" null null)
  (`parent.Effect`))

(fn `UserConstructionScript`
  (`parent.UserConstructionScript`))