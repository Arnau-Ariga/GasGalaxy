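; BP_Explosive_Nade is a throwable explosive grenade built on a parent throwable Blueprint.
; Its construction script sizes the Explosive radial force radius from EffectRange.
; Effect spawns an explosion particle at the collider, fires the radial impulse, then runs the parent effect.
; Detonate only calls the parent, with a DestroyActor node left unconnected.
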(fn `Detonate`
  (`parent.Detonate`))

(fn `Effect`
  (`GameplayStatics.SpawnEmitterAtLocation` "/Game/StarterContent/Particles/P_Explosion.P_Explosion" (`SceneComponent.K2_GetComponentLocation` (`self.ThrowableCollider`)))
  (`RadialForceComponent.FireImpulse` (`self.Explosive`))
  (`parent.Effect`))

(fn `UserConstructionScript`
  (`parent.UserConstructionScript`)
  (set `RadialForceComponent.Radius` (`self.EffectRange`) (`self.Explosive`)))