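; Game mode that populates the level with enemies at BeginPlay, spawning a random mix of penguins, walruses and snowball throwers.
; SpawnEnemies runs a fixed-count loop, placing each enemy slightly above a found location with random yaw.
; SpawnLocationFinder line-traces downward at random points across the level area, recursing until it hits an actor tagged SpawnPlatform.
; A trace that hits nothing only prints a message and does not retry.
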(event `self.ReceiveBeginPlay`
  (`self.SpawnEnemies`))

(fn `SpawnEnemies`
  (set `self.EnemySpawnCount` 20)
  (for _ (range (`self.EnemySpawnCount`))
    (bind _location (`self.SpawnLocationFinder` (0.0 0.0 0.0) (100.0 100.0)))
    (switch `int` (`KismetMathLibrary.RandomIntegerInRange` 0 2)
      (:`0`
        (bind _returnvalue (`KismetMathLibrary.MakeTransform` (+ _location (0.0 0.0 50.0)) (`KismetMathLibrary.MakeRotator` 0.0 0.0 (`KismetMathLibrary.RandomFloatInRange` -180.0 180.0))))
        (`|SpawnActorFromClass` "/Game/_GasGalaxy/Enemies/SpecificEnemies/BP_Enemy_Penguin.BP_Enemy_Penguin_C" _returnvalue "Undefined" "MultiplyWithRoot" null null))
      (:`1`
        (`|SpawnActorFromClass` "/Game/_GasGalaxy/Enemies/SpecificEnemies/BP_Enemy_Walrus.BP_Enemy_Walrus_C" _returnvalue "Undefined" "MultiplyWithRoot" null null))
      (:`2`
        (`|SpawnActorFromClass` "/Game/_GasGalaxy/Enemies/SpecificEnemies/BP_Enemy_SnowballThrower.BP_Enemy_SnowballThrower_C" _returnvalue "Undefined" "MultiplyWithRoot" null null)))))

(fn `SpawnLocationFinder`
  (params (LevelRoot :type "Vector Structure") (LevelSize :type "Vector2D Structure"))
  (returns (Location :type "Vector Structure"))
  (bind _returnvalue (+ (* (`KismetMathLibrary.MakeVector` (`KismetMathLibrary.RandomFloat`) (`KismetMathLibrary.RandomFloat`) 5000.0) (* LevelSize (100.0 100.0))) LevelRoot))
  (bind (_outhit _returnvalue_2) (`KismetSystemLibrary.LineTraceSingle` :`Start` _returnvalue :`End` (`KismetMathLibrary.MakeVector` (.x _returnvalue) (.y _returnvalue) -200.0) :`TraceChannel` "TraceTypeQuery1" :`DrawDebugType` "ForDuration"))
  (if _returnvalue_2
    (`KismetSystemLibrary.PrintString` "The Base Was Hit")
    (bind (_bblockinghit _binitialoverlap _time _distance _location _impactpoint _normal _impactnormal _physmat _hitactor) (`GameplayStatics.BreakHitResult` _outhit))
    (if (`self.ActorHasTag` _hitactor "SpawnPlatform")
      (return _location)
      (else
        (bind _location_2 (`self.SpawnLocationFinder` LevelRoot LevelSize))
        (return _location_2)))
    (else
      (`KismetSystemLibrary.PrintString` "Nothing Hit"))))

(fn `UserConstructionScript`)