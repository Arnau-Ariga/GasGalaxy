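; Enemy projectile actor that damages the player on impact.
; On hit, it applies fixed damage through the BPC_Health component of Player-tagged actors, then pushes physics-simulating components with a velocity-scaled impulse and destroys itself.
; Non-player hits skip damage but keep the impulse, while invalid targets or other EnemyProjectile-tagged actors only destroy it.
; A failed health cast leaves the projectile alive, and debug prints remain.
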(event `self.ReceiveHit`
  (params (MyComp :type "PrimitiveComponent Object Reference") (Other :type "Actor Object Reference") (OtherComp :type "PrimitiveComponent Object Reference") (bSelfMoved :type Boolean) (HitLocation :type "Vector Structure") (HitNormal :type "Vector Structure") (NormalImpulse :type "Vector Structure") (Hit :type "HitResult Structure (by ref)"))
  (`KismetSystemLibrary.PrintString` "Hit")
  (if (`KismetSystemLibrary.IsValid` Other)
    (if (`self.ActorHasTag` Other "EnemyProjectile")
      (`self.K2_DestroyActor` :!label _label) ; Then destroy this projectile
      (elif (`self.ActorHasTag` Other "Player")
        (bind _asbpc_health (cast `/Game/FirstPerson/Blueprints/BPC_Health` (`self.GetComponentByClass` Other "/Game/FirstPerson/Blueprints/BPC_Health.BPC_Health_C"))
          (:`then`
            (`/Game/FirstPerson/Blueprints/BPC_Health.TakeDamage` _asbpc_health 10.0 null null null)
            (if (`SceneComponent.IsSimulatingPhysics` OtherComp "None") :!label _label_2
              (`PrimitiveComponent.AddImpulseAtLocation` OtherComp (* (`self.GetVelocity`) 100.0) (`self.K2_GetActorLocation`) "None")
              (goto _label)
              (else
                (goto _label))))
          (:`CastFailed`
            (`KismetSystemLibrary.PrintString` "Cast Failed")))
        (else
          (`KismetSystemLibrary.PrintString` "Failure")
          (goto _label_2))))
    (else
      (goto _label))))

(fn `UserConstructionScript`)