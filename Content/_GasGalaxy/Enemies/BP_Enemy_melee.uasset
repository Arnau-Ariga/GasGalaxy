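; Melee enemy Blueprint with attack, equip and unequip events for fighting the player with a sword.
; Attack damages the player's BPC_Health on a distance check before the montage plays, then calls OnAttackEnd immediately and again on completion or interruption.
; Equip spawns a sword on the hand socket and unequip destroys it, each updating the wielding flag and notifying listeners.
; SetMovementSpeed and GetIdealRange are stubs returning zero.
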(event `/Game/_GasGalaxy/Enemies/AI/BPI_EnemyAI.Attack`
  (bind _returnvalue (`GameplayStatics.GetPlayerCharacter` 0))
  (if (<= (`self.GetDistanceTo` _returnvalue self) 250.0)
    (bind _asbpc_health (cast `/Game/PlayerHealth/BPC_Health` (`self.GetComponentByClass` _returnvalue "/Game/PlayerHealth/BPC_Health.BPC_Health_C"))
      (:`then`
        (`/Game/PlayerHealth/BPC_Health.TakeDamage` _asbpc_health (`GameplayStatics.GetPlayerCharacter` 0) 10.0 null null null))
      (:`CastFailed`
        _)))
  (`|PlayMontage` (`self.Mesh`) "/Game/Animations/Attack_Montage.Attack_Montage"
    (:`then`
      _)
    (:`OnCompleted`
      _)
    (:`OnInterrupted`
      _))
  (`self.OnAttackEnd`))

(event `/Game/_GasGalaxy/Enemies/AI/BPI_EnemyAI.EquipWeapon`
  (bind _returnvalue (`|SpawnActorFromClass` "/Game/_GasGalaxy/Weapons/BP_Weapon_Sword.BP_Weapon_Sword_C" (`self.GetTransform`) "Undefined" "MultiplyWithRoot" null null))
  (bind _output_get (set `self.WeaponActor` _returnvalue))
  (`self.K2_AttachToComponent` _output_get (`self.Mesh`) "hand_r_sword_socket" "SnapToTarget" "SnapToTarget" "SnapToTarget" true)
  (set `self.IsWieldingWeapon` true)
  (`self.OnWeaponEquipped`))

(event `/Game/_GasGalaxy/Enemies/AI/BPI_EnemyAI.UnequipWeapon`
  (`self.K2_DestroyActor` (`self.WeaponActor`))
  (set `self.IsWieldingWeapon` false)
  (`self.OnWeaponUnequipped`))

(fn `GetIdealRange`
  (returns (AttackRadius :type "Float (double-precision)") (DefendRadius :type "Float (double-precision)"))
  (return 0.0 0.0))

(fn `SetMovementSpeed`
  (params (Speed :type "/Game/_GasGalaxy/Enemies/AI/Enums/E_MovementSpeed Enum" :default "NewEnumerator0"))
  (returns (SpeedValue :type "Float (double-precision)"))
  (return 0.0))

(fn `UserConstructionScript`
  (`parent.UserConstructionScript`))