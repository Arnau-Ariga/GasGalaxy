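; Penguin enemy Blueprint, a specific enemy that performs a slide attack.
; On Attack it plays the slide montage on its mesh, then signals attack end and prints a debug string.
; That end call fires both immediately after starting the montage and again on completion or interruption.
; It overrides the ideal range with fixed attack and defend radii; a player-distance check is left unconnected.
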(event `/Game/_GasGalaxy/Enemies/AI/BPI_EnemyAI.Attack`
  (`|PlayMontage` (`self.Mesh`) "/Game/_GasGalaxy/Enemies/EnemyModels/PenguinGoodModel/Animations/penguinSlideAttackFinal_Montage.penguinSlideAttackFinal_Montage"
    (:`then`
      _)
    (:`OnCompleted`
      _)
    (:`OnInterrupted`
      _))
  (`self.OnAttackEnd`)
  (`KismetSystemLibrary.PrintString` "On Attack Ended"))

(fn `GetIdealRange`
  (returns (AttackRadius :type "Float (double-precision)") (DefendRadius :type "Float (double-precision)"))
  (return 200.0 300.0))

(fn `UserConstructionScript`
  (`parent.UserConstructionScript`))