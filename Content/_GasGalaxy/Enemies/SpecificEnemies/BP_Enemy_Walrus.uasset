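; Walrus enemy Blueprint, a melee variant that supplies its own attack, movement speeds and combat ranges, with an empty patrol route.
; Attack applies flat damage through the player's BPC_Health component when within reach, before playing the attack montage rather than on an animation notify.
; OnAttackEnd fires as soon as the montage call returns, as well as on completion or interruption.
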(event `/Game/_GasGalaxy/Enemies/AI/BPI_EnemyAI.Attack`
  (bind _returnvalue (`GameplayStatics.GetPlayerCharacter` 0))
  (if (<= (`self.GetDistanceTo` _returnvalue self) 250.0)
    (`/Game/PlayerHealth/BPC_Health.TakeDamage` (`self.GetComponentByClass` _returnvalue "/Game/PlayerHealth/BPC_Health.BPC_Health_C") _returnvalue 10.0 null null null))
  (`|PlayMontage` (`self.Mesh`) "/Game/_GasGalaxy/Enemies/EnemyModels/Walrus/Animations/walrusAttackAnim_Montage.walrusAttackAnim_Montage"
    (:`then`
      _)
    (:`OnCompleted`
      _)
    (:`OnInterrupted`
      _))
  (`self.OnAttackEnd`)
  (`KismetSystemLibrary.PrintString` "On Attack Ended"))

(fn `GetIdealRange`
  (returns (AttackRadius :type "Float (double-precision)") (DefendRadius :type "Float (double-precision)"))
  (return 200.0 300.0))

(fn `GetPatrolRoute`
  (returns (PatrolRoute :type "/Game/_GasGalaxy/Enemies/AI/BP_PatrolRoute Object Reference"))
  (return null))

(fn `SetMovementSpeed`
  (params (Speed :type "/Game/_GasGalaxy/Enemies/AI/Enums/E_MovementSpeed Enum" :default "NewEnumerator0"))
  (returns (SpeedValue :type "Float (double-precision)"))
  (bind _output_get (set `CharacterMovementComponent.MaxWalkSpeed` (select `/Game/_GasGalaxy/Enemies/AI/Enums/E_MovementSpeed` Speed :`NewEnumerator1` 150.0 :`NewEnumerator2` 200.0 :`NewEnumerator3` 300.0 :!type "Float (single-precision)") (`self.CharacterMovement`)))
  (return _output_get))

(fn `UserConstructionScript`
  (`parent.UserConstructionScript`))