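; Snowball-throwing ranged enemy that supplies its own attack, ideal range and movement speed behavior.
; Attack plays the throw montage and signals attack end with a debug print, both immediately after starting it and on completion or interruption.
; Attack and defend radii share one long range, and SetMovementSpeed ignores its input, returning zero.
; An unconnected player-proximity check never runs.
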(event `/Game/_GasGalaxy/Enemies/AI/BPI_EnemyAI.Attack`
  (`|PlayMontage` (`self.Mesh`) "/Game/_GasGalaxy/Enemies/EnemyModels/SnowballThrower/Animations/snowballThrowAttack_Montage.snowballThrowAttack_Montage"
    (:`then`
      _)
    (:`OnCompleted`
      _)
    (:`OnInterrupted`
      _))
  (`self.OnAttackEnd`)
  (`KismetSystemLibrary.PrintString` "On Attack Ended"))

(fn `GetIdealRange`
  (returns (AttackRadius :type "Float (double-precision)") (DefendRadius :type "Float (double-precision)"))
  (return 1200.0 1200.0))

(fn `SetMovementSpeed`
  (params (Speed :type "/Game/_GasGalaxy/Enemies/AI/Enums/E_MovementSpeed Enum" :default "NewEnumerator0"))
  (returns (SpeedValue :type "Float (double-precision)"))
  (return 0.0))

(fn `UserConstructionScript`
  (`parent.UserConstructionScript`))