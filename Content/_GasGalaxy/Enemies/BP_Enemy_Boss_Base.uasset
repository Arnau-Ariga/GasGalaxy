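; Base Blueprint for boss enemies, handling sword wielding and movement speed.
; EquipWeapon spawns a sword actor and snaps it to the mesh's right-hand socket, while UnequipWeapon destroys it; both update the wielding flag and notify through equipped and unequipped calls.
; SetMovementSpeed maps movement states to walk speed, with every moving state sharing one pace, and always returns zero.
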(event `/Game/_GasGalaxy/Enemies/AI/BPI_EnemyAI.EquipWeapon`
  (bind _returnvalue (`|SpawnActorFromClass` "/Game/Weapons/BP_Weapon_Sword.BP_Weapon_Sword_C" (`self.GetTransform`) "Undefined" "MultiplyWithRoot" null null))
  (bind _output_get (set `self.WeaponActor` _returnvalue))
  (`self.K2_AttachToComponent` _output_get (`self.Mesh`) "hand_r_sword_socket" "SnapToTarget" "SnapToTarget" "SnapToTarget" true)
  (set `self.IsWieldingWeapon` true)
  (`self.OnWeaponEquipped`))

(event `/Game/_GasGalaxy/Enemies/AI/BPI_EnemyAI.UnequipWeapon`
  (`self.K2_DestroyActor` (`self.WeaponActor`))
  (set `self.IsWieldingWeapon` false)
  (`self.OnWeaponUnequipped`))

(fn `SetMovementSpeed`
  (params (Speed :type "/Game/_GasGalaxy/Enemies/AI/Enums/E_MovementSpeed Enum" :default "NewEnumerator0"))
  (returns (SpeedValue :type "Float (double-precision)"))
  (set `CharacterMovementComponent.MaxWalkSpeed` (select `/Game/_GasGalaxy/Enemies/AI/Enums/E_MovementSpeed` Speed :`NewEnumerator1` 200.0 :`NewEnumerator2` 200.0 :`NewEnumerator3` 200.0 :!type "Float (single-precision)") (`self.CharacterMovement`))
  (return 0.0))

(fn `UserConstructionScript`
  (`parent.UserConstructionScript`))