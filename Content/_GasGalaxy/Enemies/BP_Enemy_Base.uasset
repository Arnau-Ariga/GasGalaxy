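; Base enemy character that holds health and supplies the movement and combat data an enemy needs.
; Any damage lowers health, clamped between zero and max, and sets a dead flag at zero with no further death handling here.
; Getters expose health, a patrol route and fixed attack and defend radii.
; A setter maps a speed state, from idle to sprinting, onto max walk speed and returns it.
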(event `self.ReceiveAnyDamage`
  (params (Damage :type "Float (single-precision)") (DamageType :type "DamageType Object Reference") (InstigatedBy :type "Controller Object Reference") (DamageCauser :type "Actor Object Reference"))
  (bind _output_get (set `self.Health` (`KismetMathLibrary.FClamp` (- (`self.Health`) Damage) 0.0 (`self.MaxHealth`))))
  (if (<= _output_get 0.0)
    (set `self.IsDead` true)))

(fn `GetCurrentHealth`
  (returns (Health :type "Float (double-precision)"))
  (return (`self.Health`)))

(fn `GetIdealRange`
  (returns (AttackRadius :type "Float (double-precision)") (DefendRadius :type "Float (double-precision)"))
  (return 150.0 350.0))

(fn `GetMaxHealth`
  (returns (MaxHealth :type "Float (double-precision)"))
  (return (`self.MaxHealth`)))

(fn `GetPatrolRoute`
  (returns (PatrolRoute :type "/Game/_GasGalaxy/Enemies/AI/BP_PatrolRoute Object Reference"))
  (return (`self.PatrolRoute`)))

(fn `SetMovementSpeed`
  (params (Speed :type "/Game/_GasGalaxy/Enemies/AI/Enums/E_MovementSpeed Enum" :default "NewEnumerator0"))
  (returns (SpeedValue :type "Float (double-precision)"))
  (bind _output_get (set `CharacterMovementComponent.MaxWalkSpeed` (select `/Game/_GasGalaxy/Enemies/AI/Enums/E_MovementSpeed` Speed :`NewEnumerator1` 100.0 :`NewEnumerator2` 300.0 :`NewEnumerator3` 500.0 :!type "Float (single-precision)") (`self.CharacterMovement`)))
  (return _output_get))

(fn `UserConstructionScript`)