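; Ranged enemy Blueprint that carries a rifle and fires projectiles at its AI attack target.
; On BeginPlay it spawns the rifle and attaches it to the right-hand socket.
; Attack signals attack end immediately, then spawns a tagged projectile aimed at the AIC_Enemy_Base controller's target.
; It also supplies equal attack and defend ranges and maps movement states to walk speeds.
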(event `self.ReceiveBeginPlay`
  (`self.EquipWeapon`))

(event `self.EquipWeapon`
  (bind _returnvalue (`|SpawnActorFromClass` "/Game/_GasGalaxy/Weapons/BP_Weapon_Rifle.BP_Weapon_Rifle_C" (`KismetMathLibrary.MakeTransform` (0.0 0.0 0.0)) "Undefined" "MultiplyWithRoot" null null))
  (bind _output_get (set `self.WeaponActor` _returnvalue))
  (`self.K2_AttachToComponent` _output_get (`self.Mesh`) "hand_r_sword_socket" "SnapToTarget" "SnapToTarget" "SnapToTarget" true)
  (set `self.IsWieldingWeapon` true)
  (`self.OnWeaponEquipped`))

(event `self.Attack`
  (bind _location (.location (`SceneComponent.K2_GetComponentToWorld` (`self.SpawnProjectileLocation`))))
  (`self.OnAttackEnd`)
  (bind _asaic_enemy_base (cast `/Game/_GasGalaxy/Enemies/AI/AIC_Enemy_Base` (`AIBlueprintHelperLibrary.GetAIController` self)))
  (bind _attacktarget (`/Game/_GasGalaxy/Enemies/AI/AIC_Enemy_Base.AttackTarget` _asaic_enemy_base)
    (:`then`
      (bind _returnvalue (`|SpawnActorFromClass` "/Game/_GasGalaxy/Enemies/BP_EnemyProjectile.BP_EnemyProjectile_C" (`KismetMathLibrary.MakeTransform` _location (`KismetMathLibrary.FindLookAtRotation` _location (`self.K2_GetActorLocation` _attacktarget)) (.scale (`SceneComponent.K2_GetComponentToWorld` (`self.SpawnProjectileLocation`)))) "Undefined" "MultiplyWithRoot" null null))
      (set `Actor.Tags` (`|MakeArray` "EnemyProjectile") _returnvalue))
    (:`else`)))

(fn `GetIdealRange`
  (returns (AttackRadius :type "Float (double-precision)") (DefendRadius :type "Float (double-precision)"))
  (return 600.0 600.0))

(fn `SetMovementSpeed`
  (params (Speed :type "/Game/_GasGalaxy/Enemies/AI/Enums/E_MovementSpeed Enum" :default "NewEnumerator0"))
  (returns (SpeedValue :type "Float (double-precision)"))
  (bind _output_get (set `CharacterMovementComponent.MaxWalkSpeed` (select `/Game/_GasGalaxy/Enemies/AI/Enums/E_MovementSpeed` Speed :`NewEnumerator1` 200.0 :`NewEnumerator2` 300.0 :`NewEnumerator3` 500.0 :!type "Float (single-precision)") (`self.CharacterMovement`)))
  (return _output_get))

(fn `UserConstructionScript`
  (`parent.UserConstructionScript`))